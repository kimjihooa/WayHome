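; Utility actor in the CartoonCelShader content that displays a configurable mesh spinning and bobbing in place.
; SetMesh applies the Mesh and Material variables to the StaticMesh component at construction and again on BeginPlay.
; Tick applies delta-scaled yaw and adds a real-time sine Z offset each frame.
; The bob is frame-rate dependent, and UpAndDownAmplitude acts as a divisor, so larger values shrink the motion.
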(event EventBeginPlay
  (CallFunction|SetMesh))

(event EventTick
  (params (DeltaSeconds :type Float%20%28single-precision%29))
  (Transformation|AddWorldRotation (Variables|Default|GetStaticMesh) (Math|Rotator|MakeRotator 0.0 0.0 (* DeltaSeconds (Variables|Default|GetRotateSpeed))) false false)
  (Transformation|AddWorldOffset (Variables|Default|GetStaticMesh) (Math|Vector|MakeVector 0.0 0.0 (/ (Math|Trig|Sin(Radians) (* (Utilities|Time|GetRealTimeSeconds) (Variables|Default|GetUp_and_Down%20Speed))) (Variables|Default|GetUp_and_Down%20Amplitude))) false false))

(fn ConstructionScript
  (CallFunction|SetMesh))

(fn SetMesh
  (bind _staticmesh (Variables|Default|GetStaticMesh))
  (Components|StaticMesh|SetStaticMesh _staticmesh (Variables|Default|GetMesh))
  (Rendering|Material|SetMaterial _staticmesh 0 (Variables|Default|GetMaterial)))