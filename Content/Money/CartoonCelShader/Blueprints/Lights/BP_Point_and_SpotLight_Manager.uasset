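; Manager that feeds the four point lights and four spot lights nearest the player pawn into MPC_Point_and_SpotLight, apparently for cel shader materials.
; Lights are gathered at BeginPlay or on each Delay-throttled Tick update, then swap-sorted by distance and clamped.
; Position, radius, color, intensity, direction and spot cone angle go into numbered vector parameters.
; Construction and BeginPlay push cull settings, and reset functions clear light slots.
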(event EventTick
  (params (DeltaSeconds :type Float%20%28single-precision%29))
  (Utilities|FlowControl|Delay (/ 1.0 (Variables|Default|GetUpdate%20rate%20in%20FPS)))
  (Utilities|FlowControl|Sequence
    (:then_0
      (if (Variables|Default|GetUse%20PointLight?)
        (if (Variables|Default|GetPoint%20Lights%20Are%20Updated%20Real%20Time?)
          (CallFunction|ResetPointLights)
          (bind _outactors (Actor|GetAllActorsOfClass "/Script/Engine.PointLight"))
          (Variables|Default|SetPointLights _outactors))
        (bind _local_point_light (CallFunction|InitializePointLights (Variables|Default|GetPointLights)))
        (bind _point_lights_clamp (CallFunction|ClampPointLights _local_point_light))
        (CallFunction|ProcessPointLights _point_lights_clamp)
        (else
          (CallFunction|ResetPointLights))))
    (:then_1
      (if (Variables|Default|GetUse%20Spotlight?)
        (if (Variables|Default|GetSpot%20Lights%20Are%20Updated%20Real%20Time?)
          (CallFunction|ResetSpotLights)
          (bind _outactors_2 (Actor|GetAllActorsOfClass "/Script/Engine.SpotLight"))
          (Variables|Default|SetSpot%20Lights _outactors_2))
        (bind _local_spot_light (CallFunction|InitializeSpotLights (Variables|Default|GetSpot%20Lights)))
        (bind _spot_lights_clamp (CallFunction|ClampSpotLights _local_spot_light))
        (CallFunction|ProcessSpotLights _spot_lights_clamp)
        (else
          (CallFunction|ResetSpotLights))))))

(event EventBeginPlay
  (Utilities|FlowControl|Sequence
    (:then_0
      (CallFunction|PointLightParameters)
      (if (Variables|Default|GetUse%20PointLight?)
        (if (not (Variables|Default|GetPoint%20Lights%20Are%20Updated%20Real%20Time?))
          (bind _outactors (Actor|GetAllActorsOfClass "/Script/Engine.PointLight"))
          (Variables|Default|SetPointLights _outactors))))
    (:then_1
      (CallFunction|SpotLightParameters)
      (if (Variables|Default|GetUse%20Spotlight?)
        (if (not (Variables|Default|GetSpot%20Lights%20Are%20Updated%20Real%20Time?))
          (bind _outactors_2 (Actor|GetAllActorsOfClass "/Script/Engine.SpotLight"))
          (Variables|Default|SetSpot%20Lights _outactors_2))))))

(fn ConstructionScript
  (Utilities|FlowControl|Sequence
    (:then_0
      (CallFunction|PointLightParameters)
      (CallFunction|ResetPointLights))
    (:then_1
      (CallFunction|SpotLightParameters)
      (CallFunction|ResetSpotLights))))

(fn InitializePointLights
  (params (Point%20Lights :type Array%20of%20Point%20Light%20Object%20References))
  (bind _returnvalue (Game|Player|GetPlayerPawn 0))
  (bind _returnvalue_2 (Transformation|GetActorLocation _returnvalue))
  (bind _output_get (LocalVariables|SetLocal%20Point%20Lights Point%20Lights))
  (for (_array_element _array_index) _output_get
    (for _index (range _array_index (Utilities|Array|LastIndex (LocalVariables|GetLocal%20Point%20Lights)))
      (if (Utilities|IsValid (Utilities|Array|Get(acopy) (LocalVariables|GetLocal%20Point%20Lights) _index))
        (if (< (Math|Vector|Distance(Vector) (Transformation|GetWorldLocation (Variables|/Script/Engine.PointLight|GetPointLightComponent (Utilities|Array|Get(acopy) (LocalVariables|GetLocal%20Point%20Lights) _index))) _returnvalue_2) (Math|Vector|Distance(Vector) _returnvalue_2 (Transformation|GetWorldLocation (Variables|/Script/Engine.PointLight|GetPointLightComponent _array_element))))
          (Utilities|Array|Swap (LocalVariables|GetLocal%20Point%20Lights) _index _array_index))
        (else
          (CallFunction|ResetPointLights)
          (Utilities|Array|RemoveItem (LocalVariables|GetLocal%20Point%20Lights) (Utilities|Array|Get(acopy) (LocalVariables|GetLocal%20Point%20Lights) _index))))))
  (return (LocalVariables|GetLocal%20Point%20Lights)))

(fn ClampPointLights
  (params (in :type Array%20of%20Point%20Light%20Object%20References))
  (bind _returnvalue (Utilities|Array|Length in))
  (if (> _returnvalue 4)
    (Utilities|Array|Resize in 4)
    (elif (== _returnvalue 0)
      (Utilities|Array|Clear in)
      (else
        (Utilities|Array|Resize in _returnvalue))))
  (return in))

(fn ProcessPointLights
  (params (Array :type Array%20of%20Point%20Light%20Object%20References))
  (if (Variables|Default|GetDebug%20Point%20Lights?)
    (for _array_element Array
      (Development|PrintString (Utilities|String|Append "Point: " (Utilities|GetDisplayName _array_element)) true true "(R=1.000000,G=0.715694,B=0.000000,A=1.000000)" (/ 1.0 (Variables|Default|GetUpdate%20rate%20in%20FPS)))
      (bind (_array_element_2 _array_index) (Utilities|Array|ForEachLoopwithBreak Array)
        (:LoopBody
          (Rendering|Material|SetVectorParameterValue "/Game/Money/CartoonCelShader/Materials/MaterialCollections/MPC_Point_and_SpotLight.MPC_Point_and_SpotLight" (Utilities|String|StringToName (Utilities|String|Append "Vector" (Utilities|String|ToString(Integer) (+ _array_index 1)))) (Utilities|Struct|MakeLinearColor (.x (Transformation|GetWorldLocation (Variables|/Script/Engine.PointLight|GetPointLightComponent _array_element_2))) (.y (Transformation|GetWorldLocation (Variables|/Script/Engine.PointLight|GetPointLightComponent _array_element_2))) (.z (Transformation|GetWorldLocation (Variables|/Script/Engine.PointLight|GetPointLightComponent _array_element_2))) (Variables|/Script/Engine.LocalLightComponent|GetAttenuationRadius (Variables|/Script/Engine.PointLight|GetPointLightComponent _array_element_2))) :!class /Script/Engine.KismetMaterialLibrary)
          (Rendering|Material|SetVectorParameterValue "/Game/Money/CartoonCelShader/Materials/MaterialCollections/MPC_Point_and_SpotLight.MPC_Point_and_SpotLight" (Utilities|String|StringToName (Utilities|String|Append "Vector" (Utilities|String|ToString(Integer) (+ _array_index 5)))) (Utilities|Struct|MakeLinearColor (.r (Rendering|Components|Light|GetLightColor (Variables|/Script/Engine.PointLight|GetPointLightComponent _array_element_2))) (.g (Rendering|Components|Light|GetLightColor (Variables|/Script/Engine.PointLight|GetPointLightComponent _array_element_2))) (.b (Rendering|Components|Light|GetLightColor (Variables|/Script/Engine.PointLight|GetPointLightComponent _array_element_2))) (Variables|/Script/Engine.LightComponentBase|GetIntensity (Variables|/Script/Engine.PointLight|GetPointLightComponent _array_element_2))) :!class /Script/Engine.KismetMaterialLibrary)
          (Rendering|Material|SetVectorParameterValue "/Game/Money/CartoonCelShader/Materials/MaterialCollections/MPC_Point_and_SpotLight.MPC_Point_and_SpotLight" (Utilities|String|StringToName (Utilities|String|Append "Vector" (Utilities|String|ToString(Integer) (+ _array_index 21)))) (Utilities|Struct|MakeLinearColor (.x (Math|Vector|GetUnitDirection(Vector) (Transformation|GetWorldLocation (Variables|/Script/Engine.PointLight|GetPointLightComponent _array_element_2)) (Transformation|GetActorLocation (Game|Player|GetPlayerPawn 0)))) (.y (Math|Vector|GetUnitDirection(Vector) (Transformation|GetWorldLocation (Variables|/Script/Engine.PointLight|GetPointLightComponent _array_element_2)) (Transformation|GetActorLocation (Game|Player|GetPlayerPawn 0)))) (.z (Math|Vector|GetUnitDirection(Vector) (Transformation|GetWorldLocation (Variables|/Script/Engine.PointLight|GetPointLightComponent _array_element_2)) (Transformation|GetActorLocation (Game|Player|GetPlayerPawn 0)))) 0.0) :!class /Script/Engine.KismetMaterialLibrary))))
    (else
      (bind (_array_element_3 _array_index_2) (Utilities|Array|ForEachLoopwithBreak Array)
        (:LoopBody
          (Rendering|Material|SetVectorParameterValue "/Game/Money/CartoonCelShader/Materials/MaterialCollections/MPC_Point_and_SpotLight.MPC_Point_and_SpotLight" (Utilities|String|StringToName (Utilities|String|Append "Vector" (Utilities|String|ToString(Integer) (+ _array_index_2 1)))) (Utilities|Struct|MakeLinearColor (.x (Transformation|GetWorldLocation (Variables|/Script/Engine.PointLight|GetPointLightComponent _array_element_3))) (.y (Transformation|GetWorldLocation (Variables|/Script/Engine.PointLight|GetPointLightComponent _array_element_3))) (.z (Transformation|GetWorldLocation (Variables|/Script/Engine.PointLight|GetPointLightComponent _array_element_3))) (Variables|/Script/Engine.LocalLightComponent|GetAttenuationRadius (Variables|/Script/Engine.PointLight|GetPointLightComponent _array_element_3))) :!class /Script/Engine.KismetMaterialLibrary)
          (Rendering|Material|SetVectorParameterValue "/Game/Money/CartoonCelShader/Materials/MaterialCollections/MPC_Point_and_SpotLight.MPC_Point_and_SpotLight" (Utilities|String|StringToName (Utilities|String|Append "Vector" (Utilities|String|ToString(Integer) (+ _array_index_2 5)))) (Utilities|Struct|MakeLinearColor (.r (Rendering|Components|Light|GetLightColor (Variables|/Script/Engine.PointLight|GetPointLightComponent _array_element_3))) (.g (Rendering|Components|Light|GetLightColor (Variables|/Script/Engine.PointLight|GetPointLightComponent _array_element_3))) (.b (Rendering|Components|Light|GetLightColor (Variables|/Script/Engine.PointLight|GetPointLightComponent _array_element_3))) (Variables|/Script/Engine.LightComponentBase|GetIntensity (Variables|/Script/Engine.PointLight|GetPointLightComponent _array_element_3))) :!class /Script/Engine.KismetMaterialLibrary)
          (Rendering|Material|SetVectorParameterValue "/Game/Money/CartoonCelShader/Materials/MaterialCollections/MPC_Point_and_SpotLight.MPC_Point_and_SpotLight" (Utilities|String|StringToName (Utilities|String|Append "Vector" (Utilities|String|ToString(Integer) (+ _array_index_2 21)))) (Utilities|Struct|MakeLinearColor (.x (Math|Vector|GetUnitDirection(Vector) (Transformation|GetWorldLocation (Variables|/Script/Engine.PointLight|GetPointLightComponent _array_element_3)) (Transformation|GetActorLocation (Game|Player|GetPlayerPawn 0)))) (.y (Math|Vector|GetUnitDirection(Vector) (Transformation|GetWorldLocation (Variables|/Script/Engine.PointLight|GetPointLightComponent _array_element_3)) (Transformation|GetActorLocation (Game|Player|GetPlayerPawn 0)))) (.z (Math|Vector|GetUnitDirection(Vector) (Transformation|GetWorldLocation (Variables|/Script/Engine.PointLight|GetPointLightComponent _array_element_3)) (Transformation|GetActorLocation (Game|Player|GetPlayerPawn 0)))) 0.0) :!class /Script/Engine.KismetMaterialLibrary))))))

(fn ResetPointLights
  (bind _linearcolor (Utilities|Struct|MakeLinearColor 0.0 0.0 0.0 0.0))
  (bind _array_index (Utilities|Array|ForEachLoopwithBreak (Variables|Default|GetPointLights))
    (:LoopBody
      (Rendering|Material|SetVectorParameterValue "/Game/Money/CartoonCelShader/Materials/MaterialCollections/MPC_Point_and_SpotLight.MPC_Point_and_SpotLight" (Utilities|String|StringToName (Utilities|String|Append "Vector" (Utilities|String|ToString(Integer) (+ _array_index 1)))) _linearcolor :!class /Script/Engine.KismetMaterialLibrary)
      (Rendering|Material|SetVectorParameterValue "/Game/Money/CartoonCelShader/Materials/MaterialCollections/MPC_Point_and_SpotLight.MPC_Point_and_SpotLight" (Utilities|String|StringToName (Utilities|String|Append "Vector" (Utilities|String|ToString(Integer) (+ _array_index 5)))) _linearcolor :!class /Script/Engine.KismetMaterialLibrary))))

(fn PointLightParameters
  (Rendering|Material|SetScalarParameterValue "/Game/Money/CartoonCelShader/Materials/MaterialCollections/MPC_Point_and_SpotLight.MPC_Point_and_SpotLight" "Point Light Cull Distance" (Variables|Default|GetPoint%20Light%20Cull%20Distance) :!class /Script/Engine.KismetMaterialLibrary)
  (Rendering|Material|SetScalarParameterValue "/Game/Money/CartoonCelShader/Materials/MaterialCollections/MPC_Point_and_SpotLight.MPC_Point_and_SpotLight" "Point Light Cull Falloff" (Variables|Default|GetPoint%20Light%20Cull%20Falloff) :!class /Script/Engine.KismetMaterialLibrary))

(fn InitializeSpotLights
  (params (Spot%20Lights :type Array%20of%20Spot%20Light%20Object%20References))
  (bind _returnvalue (Game|Player|GetPlayerPawn 0))
  (bind _returnvalue_2 (Transformation|GetActorLocation _returnvalue))
  (bind _output_get (LocalVariables|SetLocal%20Spotlights Spot%20Lights))
  (for (_array_element _array_index) _output_get
    (for _index (range _array_index (Utilities|Array|LastIndex (LocalVariables|GetLocal%20Spotlights)))
      (if (Utilities|IsValid (Utilities|Array|Get(acopy) (LocalVariables|GetLocal%20Spotlights) _index))
        (if (< (Math|Vector|Distance(Vector) (Transformation|GetWorldLocation (Variables|/Script/Engine.SpotLight|GetSpotLightComponent (Utilities|Array|Get(acopy) (LocalVariables|GetLocal%20Spotlights) _index))) _returnvalue_2) (Math|Vector|Distance(Vector) _returnvalue_2 (Transformation|GetWorldLocation (Variables|/Script/Engine.SpotLight|GetSpotLightComponent _array_element))))
          (Utilities|Array|Swap (LocalVariables|GetLocal%20Spotlights) _index _array_index))
        (else
          (CallFunction|ResetSpotLights)
          (Utilities|Array|RemoveItem (LocalVariables|GetLocal%20Spotlights) (Utilities|Array|Get(acopy) (LocalVariables|GetLocal%20Spotlights) _index))))))
  (return (LocalVariables|GetLocal%20Spotlights)))

(fn ClampSpotLights
  (params (In :type Array%20of%20Spot%20Light%20Object%20References))
  (bind _returnvalue (Utilities|Array|Length In))
  (if (> _returnvalue 4)
    (Utilities|Array|Resize In 4)
    (elif (== _returnvalue 0)
      (Utilities|Array|Clear In)
      (else
        (Utilities|Array|Resize In _returnvalue))))
  (return In))

(fn ProcessSpotLights
  (params (Array :type Array%20of%20Spot%20Light%20Object%20References))
  (if (Variables|Default|GetDebug%20Spot%20Lights?)
    (for _array_element Array
      (Development|PrintString (Utilities|String|Append "Spot: " (Utilities|GetDisplayName _array_element)) true true "(R=1.000000,G=0.715694,B=0.000000,A=1.000000)" (/ 1.0 (Variables|Default|GetUpdate%20rate%20in%20FPS)))
      (bind (_array_element_2 _array_index) (Utilities|Array|ForEachLoopwithBreak Array)
        (:LoopBody
          (Rendering|Material|SetVectorParameterValue "/Game/Money/CartoonCelShader/Materials/MaterialCollections/MPC_Point_and_SpotLight.MPC_Point_and_SpotLight" (Utilities|String|StringToName (Utilities|String|Append "Vector" (Utilities|String|ToString(Integer) (+ _array_index 9)))) (Utilities|Struct|MakeLinearColor (.x (Transformation|GetWorldLocation (Variables|/Script/Engine.SpotLight|GetSpotLightComponent _array_element_2))) (.y (Transformation|GetWorldLocation (Variables|/Script/Engine.SpotLight|GetSpotLightComponent _array_element_2))) (.z (Transformation|GetWorldLocation (Variables|/Script/Engine.SpotLight|GetSpotLightComponent _array_element_2))) (Variables|/Script/Engine.LocalLightComponent|GetAttenuationRadius (Variables|/Script/Engine.SpotLight|GetSpotLightComponent _array_element_2))) :!class /Script/Engine.KismetMaterialLibrary)
          (Rendering|Material|SetVectorParameterValue "/Game/Money/CartoonCelShader/Materials/MaterialCollections/MPC_Point_and_SpotLight.MPC_Point_and_SpotLight" (Utilities|String|StringToName (Utilities|String|Append "Vector" (Utilities|String|ToString(Integer) (+ _array_index 13)))) (Utilities|Struct|MakeLinearColor (.r (Rendering|Components|Light|GetLightColor (Variables|/Script/Engine.SpotLight|GetSpotLightComponent _array_element_2))) (.g (Rendering|Components|Light|GetLightColor (Variables|/Script/Engine.SpotLight|GetSpotLightComponent _array_element_2))) (.b (Rendering|Components|Light|GetLightColor (Variables|/Script/Engine.SpotLight|GetSpotLightComponent _array_element_2))) (Variables|/Script/Engine.LightComponentBase|GetIntensity (Variables|/Script/Engine.SpotLight|GetSpotLightComponent _array_element_2))) :!class /Script/Engine.KismetMaterialLibrary)
          (Rendering|Material|SetVectorParameterValue "/Game/Money/CartoonCelShader/Materials/MaterialCollections/MPC_Point_and_SpotLight.MPC_Point_and_SpotLight" (Utilities|String|StringToName (Utilities|String|Append "Vector" (Utilities|String|ToString(Integer) (+ _array_index 17)))) (Utilities|Struct|MakeLinearColor (.x (Math|Vector|GetForwardVector (Variables|/Script/Engine.SpotLight|GetSpotLightComponent _array_element_2))) (.y (Math|Vector|GetForwardVector (Variables|/Script/Engine.SpotLight|GetSpotLightComponent _array_element_2))) (.z (Math|Vector|GetForwardVector (Variables|/Script/Engine.SpotLight|GetSpotLightComponent _array_element_2))) (Variables|/Script/Engine.SpotLightComponent|GetOuterConeAngle (Variables|/Script/Engine.SpotLight|GetSpotLightComponent _array_element_2))) :!class /Script/Engine.KismetMaterialLibrary))))
    (else
      (bind (_array_element_3 _array_index_2) (Utilities|Array|ForEachLoopwithBreak Array)
        (:LoopBody
          (Rendering|Material|SetVectorParameterValue "/Game/Money/CartoonCelShader/Materials/MaterialCollections/MPC_Point_and_SpotLight.MPC_Point_and_SpotLight" (Utilities|String|StringToName (Utilities|String|Append "Vector" (Utilities|String|ToString(Integer) (+ _array_index_2 9)))) (Utilities|Struct|MakeLinearColor (.x (Transformation|GetWorldLocation (Variables|/Script/Engine.SpotLight|GetSpotLightComponent _array_element_3))) (.y (Transformation|GetWorldLocation (Variables|/Script/Engine.SpotLight|GetSpotLightComponent _array_element_3))) (.z (Transformation|GetWorldLocation (Variables|/Script/Engine.SpotLight|GetSpotLightComponent _array_element_3))) (Variables|/Script/Engine.LocalLightComponent|GetAttenuationRadius (Variables|/Script/Engine.SpotLight|GetSpotLightComponent _array_element_3))) :!class /Script/Engine.KismetMaterialLibrary)
          (Rendering|Material|SetVectorParameterValue "/Game/Money/CartoonCelShader/Materials/MaterialCollections/MPC_Point_and_SpotLight.MPC_Point_and_SpotLight" (Utilities|String|StringToName (Utilities|String|Append "Vector" (Utilities|String|ToString(Integer) (+ _array_index_2 13)))) (Utilities|Struct|MakeLinearColor (.r (Rendering|Components|Light|GetLightColor (Variables|/Script/Engine.SpotLight|GetSpotLightComponent _array_element_3))) (.g (Rendering|Components|Light|GetLightColor (Variables|/Script/Engine.SpotLight|GetSpotLightComponent _array_element_3))) (.b (Rendering|Components|Light|GetLightColor (Variables|/Script/Engine.SpotLight|GetSpotLightComponent _array_element_3))) (Variables|/Script/Engine.LightComponentBase|GetIntensity (Variables|/Script/Engine.SpotLight|GetSpotLightComponent _array_element_3))) :!class /Script/Engine.KismetMaterialLibrary)
          (Rendering|Material|SetVectorParameterValue "/Game/Money/CartoonCelShader/Materials/MaterialCollections/MPC_Point_and_SpotLight.MPC_Point_and_SpotLight" (Utilities|String|StringToName (Utilities|String|Append "Vector" (Utilities|String|ToString(Integer) (+ _array_index_2 17)))) (Utilities|Struct|MakeLinearColor (.x (Math|Vector|GetForwardVector (Variables|/Script/Engine.SpotLight|GetSpotLightComponent _array_element_3))) (.y (Math|Vector|GetForwardVector (Variables|/Script/Engine.SpotLight|GetSpotLightComponent _array_element_3))) (.z (Math|Vector|GetForwardVector (Variables|/Script/Engine.SpotLight|GetSpotLightComponent _array_element_3))) (Variables|/Script/Engine.SpotLightComponent|GetOuterConeAngle (Variables|/Script/Engine.SpotLight|GetSpotLightComponent _array_element_3))) :!class /Script/Engine.KismetMaterialLibrary))))))

(fn ResetSpotLights
  (bind _linearcolor (Utilities|Struct|MakeLinearColor 0.0 0.0 0.0 0.0))
  (for (_ _array_index) (Variables|Default|GetSpot%20Lights)
    (Rendering|Material|SetVectorParameterValue "/Game/Money/CartoonCelShader/Materials/MaterialCollections/MPC_Point_and_SpotLight.MPC_Point_and_SpotLight" (Utilities|String|StringToName (Utilities|String|Append "Vector" (Utilities|String|ToString(Integer) (+ _array_index 9)))) _linearcolor :!class /Script/Engine.KismetMaterialLibrary)
    (Rendering|Material|SetVectorParameterValue "/Game/Money/CartoonCelShader/Materials/MaterialCollections/MPC_Point_and_SpotLight.MPC_Point_and_SpotLight" (Utilities|String|StringToName (Utilities|String|Append "Vector" (Utilities|String|ToString(Integer) (+ _array_index 13)))) _linearcolor :!class /Script/Engine.KismetMaterialLibrary)
    (Rendering|Material|SetVectorParameterValue "/Game/Money/CartoonCelShader/Materials/MaterialCollections/MPC_Point_and_SpotLight.MPC_Point_and_SpotLight" (Utilities|String|StringToName (Utilities|String|Append "Vector" (Utilities|String|ToString(Integer) (+ _array_index 17)))) _linearcolor :!class /Script/Engine.KismetMaterialLibrary)))

(fn SpotLightParameters
  (Rendering|Material|SetScalarParameterValue "/Game/Money/CartoonCelShader/Materials/MaterialCollections/MPC_Point_and_SpotLight.MPC_Point_and_SpotLight" "Spot Light Cull Distance" (Variables|Default|GetSpot%20Light%20Cull%20Distance) :!class /Script/Engine.KismetMaterialLibrary)
  (Rendering|Material|SetScalarParameterValue "/Game/Money/CartoonCelShader/Materials/MaterialCollections/MPC_Point_and_SpotLight.MPC_Point_and_SpotLight" "Spot Light Cull Falloff" (Variables|Default|GetSpot%20Light%20Cull%20Falloff) :!class /Script/Engine.KismetMaterialLibrary))