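; BP_Rocket is a quest rocket that the player rebuilds from three collected parts: a handle and two wings.
; Picking up a part flags it and half-clears its objective through BPCQuestGiver.
; Each interaction installs the first collected, uninstalled part by enabling its mesh visibility and collision, then clears that objective.
; Once all parts are active, the rocket locks further assembly and tells the QuestManager to clear the quest.
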(event Custom|PickupPart
  (params (PartType :type E_Rocket%20Enum :default "NewEnumerator0"))
  (bind _returnvalue (Math|Conversions|ToInteger(Byte) PartType))
  (Default|HalfClearObject (Variables|Default|GetBPC_QuestGiver) "00001" _returnvalue)
  (Utilities|Array|SetArrayElem (Variables|Default|GetbIsPickup) _returnvalue true))

(event Custom|CheckAllActive
  (bind _bpc_questgiver (Variables|Default|GetBPC_QuestGiver))
  (bind _questmanager (Variables|/Game/Blueprints/Quest/BPC_QuestGiver.BPC_QuestGiver_C|GetQuestManager _bpc_questgiver))
  (if (== (Utilities|Array|FindItem (Variables|Default|GetbIsPartActive) false) -1)
    (Variables|Default|SetbIsActiated true)
    (Utilities|IsValid _questmanager
      (:Is%20Valid
        (Default|ClearQuest _questmanager))
      (:Is%20Not%20Valid
        (Development|PrintString "QuestManager Not Valid")))))

(event EventInteractwith
  (if (not (Variables|Default|GetbIsActiated))
    (bind _index (Utilities|FlowControl|ForLoopwithBreak 0 2 :!label _label)
      (:LoopBody
        (if (and (Utilities|Array|Get(acopy) (Variables|Default|GetbIsPickup) _index) (not (Utilities|Array|Get(acopy) (Variables|Default|GetbIsPartActive) _index)))
          (CallFunction|ActivatePart (Utilities|Enum|ByteToEnumE_Rocket (Math|Conversions|ToByte(Integer) _index)))
          (Default|ClearObject (Variables|Default|GetBPC_QuestGiver) "00001" _index)
          (goto _label Break)))
      (:Completed
        (CallFunction|CheckAllActive)))))

(fn ConstructionScript)

(fn ActivatePart
  (params (PartType :type E_Rocket%20Enum :default "NewEnumerator0"))
  (bind _returnvalue (Math|Conversions|ToInteger(Byte) PartType))
  (bind _handle (Variables|Default|GetHandle))
  (bind _rightwing (Variables|Default|GetRightWing))
  (bind _leftwing (Variables|Default|GetLeftWing))
  (switch Utilities|FlowControl|Switch|SwitchonE_Rocket PartType
    (:NewEnumerator0
      (Rendering|SetVisibility _handle true false)
      (Collision|SetCollisionProfileName _handle "BlockAll" true :!class /Script/Engine.PrimitiveComponent)
      (Utilities|Array|SetArrayElem (Variables|Default|GetbIsPartActive) _returnvalue true))
    (:NewEnumerator1
      (Rendering|SetVisibility _leftwing true false)
      (Collision|SetCollisionProfileName _leftwing "BlockAll" true :!class /Script/Engine.PrimitiveComponent)
      (Utilities|Array|SetArrayElem (Variables|Default|GetbIsPartActive) _returnvalue true))
    (:NewEnumerator2
      (Rendering|SetVisibility _rightwing true false)
      (Collision|SetCollisionProfileName _rightwing "BlockAll" true :!class /Script/Engine.PrimitiveComponent)
      (Utilities|Array|SetArrayElem (Variables|Default|GetbIsPartActive) _returnvalue true))))