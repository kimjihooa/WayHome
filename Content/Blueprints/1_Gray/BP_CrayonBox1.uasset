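; Crayon box that swings its lid open and launches physics crayons when BP_Character overlaps Box1.
; OpenBox plays a timeline that rolls BoxUp and unpauses a looping spawn timer created paused at BeginPlay.
; Each tick of that timer adds a simulated crayon mesh component and impulses it along the Arrow, clearing the timer once the count exceeds CrayonNum.
; Also defines a ForEachWithDelay loop macro, unused in these graphs.
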(event OnComponentBeginOverlap(Box1)
  (params (OverlappedComponent :type Primitive%20Component%20Object%20Reference) (OtherActor :type Actor%20Object%20Reference) (OtherComp :type Primitive%20Component%20Object%20Reference) (OtherBodyIndex :type Integer) (bFromSweep :type Boolean) (SweepResult :type Hit%20Result%20Structure%20%28by%20ref%29))
  (Utilities|Casting|CastToBP_Character OtherActor)
  (CallFunction|OpenBox))

(event Custom|OpenBox
  (Variables|Default|SetbIsOpening true)
  (Utilities|Time|UnpauseTimerbyHandle (Variables|Default|GetSpawnTimer))
  (bind _newtrack_0 (Timeline|BoxOpening Play)
    (:Update
      (Transformation|SetRelativeRotation (Variables|Default|GetBoxUp) (Math|Rotator|MakeRotator _newtrack_0 0.0 0.0) false false))
    (:Finished
      (Variables|Default|SetbIsOpening false)
      (Variables|Default|SetbIsOpened true))))

(event Custom|SpawnCrayon
  (if (>= (Variables|Default|GetCrayonNum) (Variables|Default|GetCurrentCrayonNum))
    (bind _returnvalue (Game|AddComponentbyClass "/Script/Engine.StaticMeshComponent" false (Math|Transform|MakeTransform "50.000000,0.000000,50.000000" "0, 0, 0" "1.000000,1.000000,1.000000")))
    (Components|StaticMesh|SetStaticMesh _returnvalue "/Game/Assets/1_Gray/Crayon/SM_Crayon.SM_Crayon")
    (Physics|SetSimulatePhysics _returnvalue true)
    (Physics|AddImpulse _returnvalue (* (Math|Rotator|GetRotationXVector (Transformation|GetWorldRotation (Variables|Default|GetArrow))) (Variables|Default|GetForce)) "None" false)
    (Math|Integer|IncrementInt (Variables|Default|GetCurrentCrayonNum))
    (else
      (Utilities|Time|ClearandInvalidateTimerbyHandle (Variables|Default|GetSpawnTimer)))))

(event EventBeginPlay
  (bind _returnvalue (Utilities|Time|SetTimerbyEvent (delegate Custom|SpawnCrayon) (Variables|Default|GetSpawnInterval) true))
  (bind _output_get (Variables|Default|SetSpawnTimer _returnvalue))
  (Utilities|Time|PauseTimerbyHandle _output_get))

(fn ConstructionScript)