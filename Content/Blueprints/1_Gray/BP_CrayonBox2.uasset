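; Interactable crayon box with two lids and a front panel that swings open once both lids are open.
; Interactwith opens whichever lid is closer to the player character, setting its flag and playing a rotation timeline, with Lid2 mirrored on pitch and yaw.
; Each lid timeline calls CheckOpen on finish, which rolls the front open when both flags are set.
; InRange and OutRange are empty.
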(event Custom|OpenBox
  (bind _newtrack_1 (Timeline|BoxOpen Play)
    (:Update
      (Transformation|SetRelativeRotation (Variables|Default|GetFront) (Math|Rotator|MakeRotator _newtrack_1 0.0 0.0) false false))))

(event Custom|OpenLid1
  (bind (_direction _x _y _z) (Timeline|LidOpen Play)
    (:Update
      (Transformation|SetRelativeRotation (Variables|Default|GetLid1) (Math|Rotator|MakeRotator _x _y _z) false false))
    (:Finished
      (CallFunction|CheckOpen))))

(event Custom|OpenLid2
  (bind (_direction _x _y _z) (Timeline|Timeline Play)
    (:Update
      (Transformation|SetRelativeRotation (Variables|Default|GetLid2) (Math|Rotator|MakeRotator _x (* _y -1.0) (* _z -1.0)) false false))
    (:Finished
      (CallFunction|CheckOpen))))

(event Custom|CheckOpen
  (if (and (Variables|Default|GetbIsLid2Opened) (Variables|Default|GetbIsLid1Opened))
    (CallFunction|OpenBox)))

(event EventOutRange)

(event EventInRange)

(event EventInteractwith
  (if (< (Math|Vector|Distance(Vector) (Transformation|GetActorLocation (Game|GetPlayerCharacter 0)) (Transformation|GetWorldLocation (Variables|Default|GetLid1))) (Math|Vector|Distance(Vector) (Transformation|GetActorLocation (Game|GetPlayerCharacter 0)) (Transformation|GetWorldLocation (Variables|Default|GetLid2))))
    (Variables|Default|SetbIsLid1Opened true)
    (CallFunction|OpenLid1)
    (else
      (Variables|Default|SetbIsLid2Opened true)
      (CallFunction|OpenLid2))))

(fn ConstructionScript)