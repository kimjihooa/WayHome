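; BP_Crayon is a crayon prop that gets a random two-tone color each time play begins.
; On BeginPlay it creates a dynamic instance of MI_Crayon and applies it to the first material slot of its static mesh.
; It then sets the FirstColor and SecondColor parameters to independently randomized RGB values, leaving the construction script empty.
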(event EventBeginPlay
  (bind _returnvalue (Rendering|Material|CreateDynamicMaterialInstance "/Game/Assets/1_Gray/Crayon/MI_Crayon.MI_Crayon" "None" "None" :!class /Script/Engine.KismetMaterialLibrary))
  (Rendering|Material|SetMaterial (Variables|Default|GetStaticMesh) 0 _returnvalue)
  (Rendering|Material|SetVectorParameterValue _returnvalue "FirstColor" (Math|Color|MakeColor (Math|Random|RandomFloat) (Math|Random|RandomFloat) (Math|Random|RandomFloat)) :!class /Script/Engine.MaterialInstanceDynamic)
  (Rendering|Material|SetVectorParameterValue _returnvalue "SecondColor" (Math|Color|MakeColor (Math|Random|RandomFloat) (Math|Random|RandomFloat) (Math|Random|RandomFloat)) :!class /Script/Engine.MaterialInstanceDynamic))

(fn ConstructionScript)