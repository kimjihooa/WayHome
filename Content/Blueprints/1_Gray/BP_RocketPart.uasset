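; BP_RocketPart is an interactable rocket component placed in the world, configured by a PartType of Handle, Left Wing or Right Wing.
; The construction script picks its static mesh from PartType, with both wings sharing the same cube mesh.
; InRange and OutRange events show and hide its widget.
; On interaction it calls ActivatePart on the referenced Rocket with its type, or prints an error if that reference is invalid.
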(event EventInRange
  (Rendering|SetVisibility (Variables|Default|GetWidget) true false))

(event EventOutRange
  (Rendering|SetVisibility (Variables|Default|GetWidget) false false))

(event EventInteractwith
  (bind _rocket (Variables|Default|GetRocket))
  (Utilities|IsValid _rocket
    (:Is%20Valid
      (Default|ActivatePart _rocket (Variables|Default|GetPartType)))
    (:Is%20Not%20Valid
      (Development|PrintString "Rocket Not Valid"))))

(fn ConstructionScript
  (bind _staticmesh (Variables|Default|GetStaticMesh))
  (switch Utilities|FlowControl|Switch|SwitchonE_Rocket (Variables|Default|GetPartType)
    (:NewEnumerator0
      (Components|StaticMesh|SetStaticMesh _staticmesh "/Game/Money/CartoonCelShader/Meshes/PromoMesh/SM_MaterialSphere.SM_MaterialSphere"))
    (:NewEnumerator1
      (Components|StaticMesh|SetStaticMesh _staticmesh "/Game/Money/CartoonCelShader/Meshes/PromoMesh/SM_Cube_01.SM_Cube_01"))
    (:NewEnumerator2
      (Components|StaticMesh|SetStaticMesh _staticmesh "/Game/Money/CartoonCelShader/Meshes/PromoMesh/SM_Cube_01.SM_Cube_01"))))