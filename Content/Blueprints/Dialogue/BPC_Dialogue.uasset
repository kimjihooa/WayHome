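; Dialogue component that opens a dialogue UI and tracks which data table row its conversation uses.
; StartDialogue creates a WB_Dialogue widget with the speaker name, row name, data table and a self-reference, then adds it to the viewport.
; EndDialogue stores the row, table and end flag passed to it and clears the widget reference, without removing the widget itself.
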(event Custom|Event%20EndDialogue
  (params (RowName :type Name) (DataTable :type Data%20Table%20Object%20Reference) (bEndDialogue :type Boolean))
  (Variables|Default|SetRow%20Name RowName)
  (Variables|Default|SetData%20Table DataTable)
  (Variables|Default|SetbEndDialogue bEndDialogue)
  (Variables|Default|SetDialogueWidget 0))

(event EventStartDialogue
  ;[1 1 1] On Dialogue Start
  (bind _returnvalue (UserInterface|CreateWidget "/Game/Blueprints/Dialogue/WB_Dialogue.WB_Dialogue_C" 0 (Utilities|Text|ToText(Name) (Variables|Default|GetName)) (Variables|Default|GetRow%20Name) (Variables|Default|GetData%20Table) self))
  (bind _output_get (Variables|Default|SetDialogueWidget _returnvalue))
  (UserInterface|Viewport|AddtoViewport _output_get 0))