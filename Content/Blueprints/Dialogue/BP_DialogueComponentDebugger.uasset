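; Debug Blueprint that exercises the BPCDialogue component, printing strings to show which dialogue events and option choices fire.
; Interacting starts dialogue and calls its dialogue event.
; Handlers bound on BeginPlay swap themselves by unbinding and rebinding: the first option advances to a second option set, while the other ends dialogue.
; The branch binding a third option set is disconnected, and range events are empty.
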(event Custom|SecondOptions
  (params (OptionIndex :type Integer))
  ;[0.5718 1 0.9701] Secon Button Event 1
  (switch int OptionIndex
    (:0
      (Development|PrintString "A"))
    (:1
      (Development|PrintString "B"))))

(event Custom|ThirdOptions
  (params (OptionIndex :type Integer))
  ;[0.5718 1 0.9701] Second Button Event 2
  (switch int OptionIndex
    (:0
      (Development|PrintString "a"))
    (:1
      (Development|PrintString "b"))))

(event Custom|FirstDialogueEvent
  (Development|PrintString "HeHe")
  (EventDispatchers|UnbindallEventsfromOnDialogueEvent (Variables|Default|GetBPC_Dialogue))
  (EventDispatchers|BindEventtoOnDialogueEvent (Variables|Default|GetBPC_Dialogue) (delegate Custom|SecondDialogueEvent)))

(event Custom|SecondDialogueEvent
  (Development|PrintString "Jal Dwen Da"))

(event Custom|FirstOptions
  (params (OptionIndex :type Integer))
  ;[0.5718 1 0.9701] First Button Event
  (switch int OptionIndex
    (:Default
      (Development|PrintString "Option Out Of Range"))
    (:0
      (Development|PrintString "1")
      (EventDispatchers|UnbindallEventsfromOnOptionEvent (Variables|Default|GetBPC_Dialogue))
      ;[0.5718 1 0.9701] Secon Button Event 1
      (EventDispatchers|BindEventtoOnOptionEvent (Variables|Default|GetBPC_Dialogue) (delegate Custom|SecondOptions)))
    (:1
      ;;[0.6336 1 0.9095] End Dialogue Button
      (Default|EndDialogue (Variables|/Game/Blueprints/Dialogue/BPC_Dialogue.BPC_Dialogue_C|GetDialogueWidget (Variables|Default|GetBPC_Dialogue))))))

(event EventBeginPlay
  (Utilities|FlowControl|Sequence
    (:then_0
      ;[0.5718 1 0.9701] First Button Event
      (EventDispatchers|BindEventtoOnOptionEvent (Variables|Default|GetBPC_Dialogue) (delegate Custom|FirstOptions)))
    (:then_1
      (EventDispatchers|BindEventtoOnDialogueEvent (Variables|Default|GetBPC_Dialogue) (delegate Custom|FirstDialogueEvent)))))

(event EventOutRange)

(event EventInteractwith
  (bind _bpc_dialogue (Variables|Default|GetBPC_Dialogue))
  ;[1 1 1] Basic Dialogue
  (Default|StartDialogue _bpc_dialogue)
  (Default|CallOnDialogueEvent _bpc_dialogue))

(event EventInRange)

(fn ConstructionScript)