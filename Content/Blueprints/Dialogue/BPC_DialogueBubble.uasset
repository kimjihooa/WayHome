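; Actor component that shows a screen-space dialogue bubble on its owner while a BP_Character is within range.
; On BeginPlay it adds a widget component hosting WB_DialogueBubble, fed by a DataTable row, and a trigger sphere sized by BubbleRange.
; Sphere overlaps start and stop the bubble.
; If StopOnDialogue is set, entering range also binds the owner's BPC_Dialogue start event to stop the bubble.
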(event Custom|StartDialogue
  (params (OverlappedComponent :type Primitive%20Component%20Object%20Reference) (OtherActor :type Actor%20Object%20Reference) (OtherComp :type Primitive%20Component%20Object%20Reference) (OtherBodyIndex :type Integer) (bFromSweep :type Boolean) (SweepResult :type Hit%20Result%20Structure%20%28by%20ref%29))
  (bind _dialoguecomponent (Variables|Default|GetDialogueComponent))
  (Utilities|Casting|CastToBP_Character OtherActor)
  (Default|StartDialogue (Variables|Default|GetBubbleWidget))
  (if (Variables|Default|GetbStopOnDialogue)
    (Utilities|IsValid _dialoguecomponent
      (:Is%20Valid
        (EventDispatchers|BindEventtoOnDialogueStart _dialoguecomponent (delegate Custom|StopOnDialogue))))))

(event Custom|StopDialogue
  (params (OverlappedComponent :type Primitive%20Component%20Object%20Reference) (OtherActor :type Actor%20Object%20Reference) (OtherComp :type Primitive%20Component%20Object%20Reference) (OtherBodyIndex :type Integer))
  (Utilities|Casting|CastToBP_Character OtherActor)
  (Default|StopDialogue (Variables|Default|GetBubbleWidget) (Variables|Default|GetbResetDialogue)))

(event Custom|StopOnDialogue
  (Default|StopDialogue (Variables|Default|GetBubbleWidget) (Variables|Default|GetbResetDialogue)))

(event EventBeginPlay
  (bind _returnvalue (Components|GetOwner))
  (Utilities|IsValid _returnvalue
    (:Is%20Valid
      (Variables|Default|SetOwner _returnvalue)
      (Utilities|FlowControl|Sequence
        (:then_0
          (bind _returnvalue_2 (Game|AddComponentbyClass (Variables|Default|GetOwner) "/Script/UMG.WidgetComponent" false (Math|Transform|MakeTransform (Variables|Default|GetWidgetLocation) "0, 0, 0" "1.000000,1.000000,1.000000")))
          (bind _output_get (Variables|Default|SetWidetComponent _returnvalue_2))
          (Transformation|AttachComponentToComponent _output_get (Variables|/Script/Engine.Actor|GetRootComponent (Variables|Default|GetOwner)) "None" "KeepRelative" "KeepRelative" "KeepRelative" true)
          (bind _returnvalue_3 (UserInterface|CreateWidget "/Game/Blueprints/Dialogue/WB_DialogueBubble.WB_DialogueBubble_C" 0 (Variables|Default|GetRowName) (Variables|Default|GetDataTable)))
          (bind _output_get_2 (Variables|Default|SetBubbleWidget _returnvalue_3))
          (UserInterface|SetWidget (Variables|Default|GetWidetComponent) _output_get_2)
          (Class|WidgetComponent|SetWidgetSpace (Variables|Default|GetWidetComponent) "Screen")
          (Class|WidgetComponent|SetDrawSize (Variables|Default|GetWidetComponent) "(X=1000.000000,Y=500.000000)"))
        (:then_1
          (bind _returnvalue_4 (Game|AddComponentbyClass (Variables|Default|GetOwner) "/Script/Engine.SphereComponent" true))
          (bind _output_get_3 (Variables|Default|SetSphereCollision _returnvalue_4))
          (Transformation|AttachComponentToComponent _output_get_3 (Variables|/Script/Engine.Actor|GetRootComponent (Variables|Default|GetOwner)) "None" "KeepRelative" "KeepRelative" "KeepRelative" true)
          (Collision|BindEventtoOnComponentBeginOverlap (Variables|Default|GetSphereCollision) (delegate Custom|StartDialogue))
          (Collision|BindEventtoOnComponentEndOverlap (Variables|Default|GetSphereCollision) (delegate Custom|StopDialogue))
          (Components|Sphere|SetSphereRadius (Variables|Default|GetSphereCollision) (Variables|Default|GetBubbleRange) true))
        (:then_2
          (Utilities|IsValid (Actor|GetComponentbyClass (Variables|Default|GetOwner) "/Game/Blueprints/Dialogue/BPC_Dialogue.BPC_Dialogue_C")
            (:Is%20Valid
              (Variables|Default|SetDialogueComponent (Actor|GetComponentbyClass (Variables|Default|GetOwner) "/Game/Blueprints/Dialogue/BPC_Dialogue.BPC_Dialogue_C")))))))))