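; BP_Dialogue is an interactable actor that offers both a proximity speech bubble and a full dialogue.
; When ShowBubble is set, a WHCharacter entering the sphere shows and starts the WB_DialogueBubble widget; leaving hides, pauses and resets it.
; Interacting starts BPCDialogue, configured from instance variables in the construction script, then runs the same bubble-hiding path, as does EndDialogueBubble.
; Bubble and main dialogue each take their own data table and row name.
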(event OnComponentBeginOverlap(Sphere)
  (params (OverlappedComponent :type Primitive%20Component%20Object%20Reference) (OtherActor :type Actor%20Object%20Reference) (OtherComp :type Primitive%20Component%20Object%20Reference) (OtherBodyIndex :type Integer) (bFromSweep :type Boolean) (SweepResult :type Hit%20Result%20Structure%20%28by%20ref%29))
  (if (Variables|Default|GetbShowBubble)
    (Utilities|Casting|CastToWHCharacter OtherActor)
    (Rendering|SetVisibility (Variables|Default|GetWidget) true true)
    (Default|StartDialogue (Variables|Default|GetDialogueBubble))))

(event OnComponentEndOverlap(Sphere)
  (params (OverlappedComponent :type Primitive%20Component%20Object%20Reference) (OtherActor :type Actor%20Object%20Reference) (OtherComp :type Primitive%20Component%20Object%20Reference) (OtherBodyIndex :type Integer))
  (bind _dialoguebubble (Variables|Default|GetDialogueBubble))
  (if (Variables|Default|GetbShowBubble)
    (Utilities|Casting|CastToWHCharacter OtherActor)
    (Rendering|SetVisibility (Variables|Default|GetWidget) false true)
    (Default|PauseDialogue (Variables|Default|GetDialogueBubble))
    (Variables|/Game/Blueprints/Dialogue/WB_DialogueBubble.WB_DialogueBubble_C|SetRowName _dialoguebubble (Variables|Default|GetBubbleRowName))
    (Variables|/Game/Blueprints/Dialogue/WB_DialogueBubble.WB_DialogueBubble_C|SetDataTable _dialoguebubble (Variables|Default|GetBubbleDataTable))
    (Variables|/Game/Blueprints/Dialogue/WB_DialogueBubble.WB_DialogueBubble_C|SetDelay _dialoguebubble (Variables|Default|GetBubbleDelay))
    (Variables|/Game/Blueprints/Dialogue/WB_DialogueBubble.WB_DialogueBubble_C|SetbEndDialogue _dialoguebubble false)))

(event Custom|EndDialogueBubble
  (bind _dialoguebubble (Variables|Default|GetDialogueBubble))
  (if (Variables|Default|GetbShowBubble)
    (Utilities|Casting|CastToWHCharacter (stale OnComponentEndOverlap(Sphere) OtherActor))
    (Rendering|SetVisibility (Variables|Default|GetWidget) false true)
    (Default|PauseDialogue (Variables|Default|GetDialogueBubble))
    (Variables|/Game/Blueprints/Dialogue/WB_DialogueBubble.WB_DialogueBubble_C|SetRowName _dialoguebubble (Variables|Default|GetBubbleRowName))
    (Variables|/Game/Blueprints/Dialogue/WB_DialogueBubble.WB_DialogueBubble_C|SetDataTable _dialoguebubble (Variables|Default|GetBubbleDataTable))
    (Variables|/Game/Blueprints/Dialogue/WB_DialogueBubble.WB_DialogueBubble_C|SetDelay _dialoguebubble (Variables|Default|GetBubbleDelay))
    (Variables|/Game/Blueprints/Dialogue/WB_DialogueBubble.WB_DialogueBubble_C|SetbEndDialogue _dialoguebubble false)))

(event EventBeginPlay
  (Rendering|SetVisibility (Variables|Default|GetWidget) false true)
  (bind _aswb_dialogue_bubble (Utilities|Casting|CastToWB_DialogueBubble (UserInterface|GetWidget (Variables|Default|GetWidget))))
  (Variables|Default|SetDialogueBubble _aswb_dialogue_bubble)
  (Variables|/Game/Blueprints/Dialogue/WB_DialogueBubble.WB_DialogueBubble_C|SetRowName (Variables|Default|GetDialogueBubble) (Variables|Default|GetBubbleRowName))
  (Variables|/Game/Blueprints/Dialogue/WB_DialogueBubble.WB_DialogueBubble_C|SetDataTable (Variables|Default|GetDialogueBubble) (Variables|Default|GetBubbleDataTable))
  (Variables|/Game/Blueprints/Dialogue/WB_DialogueBubble.WB_DialogueBubble_C|SetDelay (Variables|Default|GetDialogueBubble) (Variables|Default|GetBubbleDelay))
  (Variables|/Game/Blueprints/Dialogue/WB_DialogueBubble.WB_DialogueBubble_C|SetDialogueActor (Variables|Default|GetDialogueBubble) self)
  (Variables|/Game/Blueprints/Dialogue/WB_DialogueBubble.WB_DialogueBubble_C|SetbEndDialogue (Variables|Default|GetDialogueBubble) false))

(event Collision|EventActorBeginOverlap
  (params (OtherActor :type Actor%20Object%20Reference)))

(event EventTick
  (params (DeltaSeconds :type Float%20%28single-precision%29)))

(event EventOutRange)

(event EventInteractwith
  (bind _dialoguebubble (Variables|Default|GetDialogueBubble))
  (Class|DialogueComponent|StartDialogue (Variables|Default|GetBPC_Dialogue))
  (if (Variables|Default|GetbShowBubble)
    (Utilities|Casting|CastToWHCharacter (stale OnComponentEndOverlap(Sphere) OtherActor))
    (Rendering|SetVisibility (Variables|Default|GetWidget) false true)
    (Default|PauseDialogue (Variables|Default|GetDialogueBubble))
    (Variables|/Game/Blueprints/Dialogue/WB_DialogueBubble.WB_DialogueBubble_C|SetRowName _dialoguebubble (Variables|Default|GetBubbleRowName))
    (Variables|/Game/Blueprints/Dialogue/WB_DialogueBubble.WB_DialogueBubble_C|SetDataTable _dialoguebubble (Variables|Default|GetBubbleDataTable))
    (Variables|/Game/Blueprints/Dialogue/WB_DialogueBubble.WB_DialogueBubble_C|SetDelay _dialoguebubble (Variables|Default|GetBubbleDelay))
    (Variables|/Game/Blueprints/Dialogue/WB_DialogueBubble.WB_DialogueBubble_C|SetbEndDialogue _dialoguebubble false)))

(event EventInRange)

(fn ConstructionScript
  (bind _bpc_dialogue (Variables|Default|GetBPC_Dialogue))
  (Variables|/Game/Blueprints/Dialogue/BPC_Dialogue.BPC_Dialogue_C|SetName _bpc_dialogue (Variables|Default|GetName))
  (Variables|/Game/Blueprints/Dialogue/BPC_Dialogue.BPC_Dialogue_C|SetRow%20Name _bpc_dialogue (Variables|Default|GetRow%20Name))
  (Variables|/Game/Blueprints/Dialogue/BPC_Dialogue.BPC_Dialogue_C|SetData%20Table _bpc_dialogue (Variables|Default|GetData%20Table)))