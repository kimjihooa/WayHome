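; BPC_Painter is a component that lets its owning actor paint BP_PaintableCharacter actors it hits.
; On BeginPlay it sets the owner's static mesh to the PainterBlockAll collision profile and binds to its hit event.
; A hit on a paintable character calls its Paint function with the impact point, normal, color and a fixed brush scale.
; A CanPaint flag and timer then enforce a cooldown between paints.
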(event Custom|OnPaintHit
  (params (HitComponent :type Primitive%20Component%20Object%20Reference) (OtherActor :type Actor%20Object%20Reference) (OtherComp :type Primitive%20Component%20Object%20Reference) (NormalImpulse :type Vector) (Hit :type Hit%20Result%20Structure%20%28by%20ref%29))
  (bind (_bblockinghit _binitialoverlap _time _distance _location _impactpoint _normal _impactnormal) (Collision|BreakHitResult Hit))
  (if (Variables|Default|GetbCanPaint)
    (Development|PrintString (Utilities|GetDisplayName OtherComp))
    (bind _asbp_paintable_character (Utilities|Casting|CastToBP_PaintableCharacter OtherActor))
    (Default|Paint _asbp_paintable_character _impactpoint _impactnormal (Math|Conversions|ToVector(LinearColor) (Math|Conversions|ToLinearColor(Color) (Variables|Default|GetPaintColor))) 4e+01 0.0)
    (Variables|Default|SetbCanPaint false)
    (Utilities|Time|SetTimerbyFunctionName 0 "ResetPaint" (Variables|Default|GetCooltime))))

(event EventBeginPlay
  (bind _returnvalue (Components|GetOwner))
  (bind _returnvalue_2 (Actor|GetComponentbyClass _returnvalue "/Script/Engine.StaticMeshComponent"))
  (Utilities|IsValid _returnvalue_2
    (:Is%20Valid
      (bind _output_get (Variables|Default|SetOriginalMesh _returnvalue_2))
      (Collision|SetCollisionProfileName _output_get "PainterBlockAll" true :!class /Script/Engine.PrimitiveComponent)
      (Collision|BindEventtoOnComponentHit (Variables|Default|GetOriginalMesh) (delegate Custom|OnPaintHit)))))

(fn ResetPaint
  (Variables|Default|SetbCanPaint true))