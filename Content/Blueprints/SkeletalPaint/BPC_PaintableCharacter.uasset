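; Character component that lets brush strokes be painted onto the owner's skeletal mesh through render targets.
; BeginPlay adds an orthographic, show-only scene capture targeting UnwrapRT.
; Each Paint call briefly swaps material slot 0 to M_Unwrap and captures the mesh, then draws M_PaintTexture into MaskRT using that capture and brush parameters.
; Render target creation is disconnected, so both targets must already exist.
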(event EventBeginPlay
  (bind _returnvalue (Components|GetOwner))
  (Utilities|FlowControl|Sequence
    (:then_2
      (bind _returnvalue_2 (Game|AddComponentbyClass _returnvalue "/Script/Engine.SceneCaptureComponent2D" false))
      (bind _output_get (Variables|Default|SetCaptureComponent _returnvalue_2))
      (Transformation|AttachComponentToComponent _output_get (Variables|/Script/Engine.Actor|GetRootComponent _returnvalue) "None" "KeepRelative" "KeepRelative" "KeepRelative" true)
      (Transformation|SetRelativeTransform _output_get (Math|Transform|MakeTransform "0.000000,0.000000,10.000000" "-90.000000,-90.000000,0.000000") false false)
      (Variables|/Script/Engine.SceneCaptureComponent2D|SetProjectionType _returnvalue_2 "Orthographic")
      (Variables|/Script/Engine.SceneCaptureComponent2D|SetOrthoWidth _output_get (Math|Conversions|ToFloat(Integer) (Variables|Default|GetUnwrapRes)))
      (Variables|/Script/Engine.SceneCaptureComponent2D|SetTextureTarget _output_get (Variables|Default|GetUnwrapRT))
      (Variables|/Script/Engine.SceneCaptureComponent|SetPrimitiveRenderMode _returnvalue_2 "PRM_UseShowOnlyList")
      (Variables|/Script/Engine.SceneCaptureComponent|SetbCaptureEveryFrame _returnvalue_2 false)
      (Variables|/Script/Engine.SceneCaptureComponent|SetbCaptureOnMovement _returnvalue_2 false))))

(fn Paint
  (params (Position :type Vector) (Normal :type Vector) (PaintColor :type Color%20Structure) (BrushScale :type Float%20%28double-precision%29) (BrushRotation :type Float%20%28double-precision%29) (BtushTexture :type Texture%20Object%20Reference))
  (CallFunction|Unwrap)
  (bind _returnvalue (Rendering|Material|CreateDynamicMaterialInstance "/Game/Blueprints/SkeletalPaint/M_PaintTexture.M_PaintTexture" "None" "None" :!class /Script/Engine.KismetMaterialLibrary))
  (Rendering|Material|SetVectorParameterValue _returnvalue "Position" (Math|Conversions|ToLinearColor(Vector) Position) :!class /Script/Engine.MaterialInstanceDynamic)
  (Rendering|Material|SetVectorParameterValue _returnvalue "Normal" (Math|Conversions|ToLinearColor(Vector) Normal) :!class /Script/Engine.MaterialInstanceDynamic)
  (Rendering|Material|SetVectorParameterValue _returnvalue "PaintColor" (Math|Conversions|ToLinearColor(Color) PaintColor) :!class /Script/Engine.MaterialInstanceDynamic)
  (Rendering|Material|SetScalarParameterValue _returnvalue "BrushScale" BrushScale :!class /Script/Engine.MaterialInstanceDynamic)
  (Rendering|Material|SetScalarParameterValue _returnvalue "BrushRotation" BrushRotation :!class /Script/Engine.MaterialInstanceDynamic)
  (Rendering|Material|SetTextureParameterValue _returnvalue "BrushTexture" BtushTexture)
  (Rendering|Material|SetTextureParameterValue _returnvalue "UnwrapTexture" (Variables|Default|GetUnwrapRT))
  (Rendering|DrawMaterialtoRenderTarget (Variables|Default|GetMaskRT) _returnvalue))

(fn Unwrap
  (bind _returnvalue (Components|GetOwner))
  (bind _capturecomponent (Variables|Default|GetCaptureComponent))
  (bind (_ascharacter _bsuccess) (Utilities|Casting|CastToCharacter _returnvalue))
  (bind _mesh (Variables|/Script/Engine.Character|GetMesh _ascharacter))
  (if _bsuccess
    (Transformation|SetWorldRotation _capturecomponent "-90.000000,-90.000000,0.000000" false false)
    (Rendering|SceneCapture|ShowOnlyComponent _capturecomponent _mesh)
    (Variables|Default|SetOriginalMaterial (Rendering|Material|GetMaterial _mesh 0))
    (Rendering|Material|SetMaterial _mesh 0 "/Game/Blueprints/SkeletalPaint/M_Unwrap.M_Unwrap")
    (Rendering|SceneCapture|CaptureScene (Variables|Default|GetCaptureComponent) :!class /Script/Engine.SceneCaptureComponent2D)
    (Rendering|Material|SetMaterial _mesh 0 (Variables|Default|GetOriginalMaterial))
    (else
      (Development|PrintString "Not Chaacter"))))