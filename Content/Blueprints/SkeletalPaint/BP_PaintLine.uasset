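; BP_PaintLine is a placeable emitter that paints skeletal characters along a line trace from its Arrow component.
; On BeginPlay a timer, optionally looping, fires a long Visibility trace along the arrow's forward vector.
; Hit actors with a BPC_PaintableCharacter component receive a Paint call at the impact point and normal, with random color, brush size and rotation.
; Debug drawing shows the trace and hit normal.
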(event Custom|Paint
  (bind _arrow (Variables|Default|GetArrow))
  (bind _returnvalue (Transformation|GetWorldLocation _arrow))
  (bind (_outhit _returnvalue_2) (Collision|LineTraceByChannel _returnvalue (+ _returnvalue (* (Math|Vector|GetForwardVector _arrow) 1e+04)) "TraceTypeQuery1" false 0 "ForOneFrame" true "(R=1.000000,G=0.000000,B=0.000000,A=1.000000)" "(R=0.000000,G=1.000000,B=0.000000,A=1.000000)" (Variables|Default|GetLoopTime)))
  (if _returnvalue_2
    (Utilities|IsValid (.HitActor (Collision|BreakHitResult _outhit))
      (:Is%20Valid
        (Utilities|IsValid (Actor|GetComponentbyClass (.HitActor (Collision|BreakHitResult _outhit)) "/Game/Blueprints/SkeletalPaint/BPC_PaintableCharacter.BPC_PaintableCharacter_C")
          (:Is%20Valid
            (Default|Paint (Actor|GetComponentbyClass (.HitActor (Collision|BreakHitResult _outhit)) "/Game/Blueprints/SkeletalPaint/BPC_PaintableCharacter.BPC_PaintableCharacter_C") (.ImpactPoint (Collision|BreakHitResult _outhit)) (.ImpactNormal (Collision|BreakHitResult _outhit)) (.OutItem (Utilities|Array|Random (Variables|Default|GetColorList))) (Math|Random|RandomFloatinRange (Variables|Default|GetMinBrushSize) (Variables|Default|GetMaxBrushSize)) (Math|Random|RandomFloatinRange (Variables|Default|GetMinBrushRotation) (Variables|Default|GetMaxBrushRotation)) (Variables|Default|GetBrushTexture))
            (Rendering|Debug|DrawDebugArrow (.ImpactPoint (Collision|BreakHitResult _outhit)) (+ (.ImpactPoint (Collision|BreakHitResult _outhit)) (* (.ImpactNormal (Collision|BreakHitResult _outhit)) 5e+01)) 0.0 "(R=1.000000,G=0.000000,B=0.000000,A=1.000000)" (Variables|Default|GetLoopTime) 0.0)))))))

(event EventBeginPlay
  (Utilities|Time|SetTimerbyEvent (delegate Custom|Paint) (Variables|Default|GetLoopTime) (Variables|Default|GetbLoop)))

(fn ConstructionScript)