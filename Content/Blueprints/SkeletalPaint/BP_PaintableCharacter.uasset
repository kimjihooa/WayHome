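; Character Blueprint whose skeletal mesh can be painted at a world position and normal with a given color, brush scale and rotation.
; Paint first calls Unwrap, which briefly swaps material slot 0 to M_Unwrap for a mesh-only scene capture, then restores the materials.
; It then draws a dynamic M_PaintTexture brush material into CRT_Mask, which is cleared on BeginPlay.
; A camera line-trace paint trigger exists but is unconnected.
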(event EventBeginPlay
  (Rendering|ClearRenderTarget2D "/Game/Blueprints/SkeletalPaint/CRT_Mask.CRT_Mask"))

(event Input|KeyboardEvents|E
  (params (Key :type Key%20Structure :default "None")))

(fn ConstructionScript)

(fn Unwrap
  (bind _scenecapturecomponent2d (Variables|Components|GetSceneCaptureComponent2D))
  (bind _mesh (Variables|Character|GetMesh))
  (Transformation|SetWorldRotation _scenecapturecomponent2d "-90.000000,-90.000000,0.000000" false false)
  (Rendering|SceneCapture|ShowOnlyComponent _scenecapturecomponent2d _mesh)
  (Variables|Default|SetMaterials (Rendering|Material|GetMaterials _mesh))
  (Rendering|Material|SetMaterial (Variables|Character|GetMesh) 0 "/Game/Blueprints/SkeletalPaint/M_Unwrap.M_Unwrap")
  (Rendering|SceneCapture|CaptureScene (Variables|Components|GetSceneCaptureComponent2D) :!class /Script/Engine.SceneCaptureComponent2D)
  (for (_array_element _array_index) (Variables|Default|GetMaterials)
    (Rendering|Material|SetMaterial (Variables|Character|GetMesh) _array_index _array_element)))

(fn Paint
  (params (Position :type Vector) (Normal :type Vector) (PaintColor :type Vector) (BrushScale :type Float%20%28double-precision%29) (BrushRotation :type Float%20%28double-precision%29))
  (CallFunction|Unwrap)
  (bind _returnvalue (Rendering|Material|CreateDynamicMaterialInstance "/Game/Blueprints/SkeletalPaint/M_PaintTexture.M_PaintTexture" "None" "None" :!class /Script/Engine.KismetMaterialLibrary))
  (Rendering|Material|SetVectorParameterValue _returnvalue "Position" (Math|Conversions|ToLinearColor(Vector) Position) :!class /Script/Engine.MaterialInstanceDynamic)
  (Rendering|Material|SetVectorParameterValue _returnvalue "Normal" (Math|Conversions|ToLinearColor(Vector) Normal) :!class /Script/Engine.MaterialInstanceDynamic)
  (Rendering|Material|SetVectorParameterValue _returnvalue "PaintColor" (Math|Conversions|ToLinearColor(Vector) PaintColor) :!class /Script/Engine.MaterialInstanceDynamic)
  (Rendering|Material|SetScalarParameterValue _returnvalue "BrushScale" BrushScale :!class /Script/Engine.MaterialInstanceDynamic)
  (Rendering|Material|SetScalarParameterValue _returnvalue "BrushRotation" BrushRotation :!class /Script/Engine.MaterialInstanceDynamic)
  (Rendering|DrawMaterialtoRenderTarget "/Game/Blueprints/SkeletalPaint/CRT_Mask.CRT_Mask" _returnvalue))