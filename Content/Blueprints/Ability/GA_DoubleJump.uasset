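; Gameplay ability that gives the avatar character an upward double-jump boost.
; On activation, if CanDoubleJump is set, it launches the character by JumpVelocity, added to current velocity, and clears the flag.
; A WaitInputRelease task restores the flag and ends the ability when input is released, with no grounded or landing check.
; If the flag is clear on activation, the ability ends immediately.
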(event Ability|EventActivateAbility
  (if (Variables|Default|GetbCanDoubleJump)
    (bind _ascharacter (Utilities|Casting|CastToCharacter (Ability|GetAvatarActorfromActorInfo)))
    (Character|LaunchCharacter _ascharacter (Math|Vector|MakeVector 0.0 0.0 (Variables|Default|GetJumpVelocity)) false false)
    (Variables|Default|SetbCanDoubleJump false)
    (Ability|Tasks|WaitInputRelease true
      (:OnRelease
        (Variables|Default|SetbCanDoubleJump true)
        (Ability|EndAbility)))
    (else
      (Ability|EndAbility))))