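; GA_Glide is a gameplay ability that lets a character glide while the input is held.
; On activation it saves the avatar's gravity scale and air control, applies glide values, and zeroes vertical velocity.
; It waits for input release to end, and restores the saved movement values when the ability ends.
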(event Ability|EventActivateAbility
  (bind _ascharacter (Utilities|Casting|CastToCharacter (Ability|GetAvatarActorfromActorInfo)))
  (Variables|Default|SetOriginal%20Gravity%20Scale (Variables|/Script/Engine.CharacterMovementComponent|GetGravityScale (Variables|/Script/Engine.Character|GetCharacterMovement _ascharacter)))
  (Variables|Default|SetOriginal%20Air%20Control (Variables|/Script/Engine.CharacterMovementComponent|GetAirControl (Variables|/Script/Engine.Character|GetCharacterMovement _ascharacter)))
  (Variables|/Script/Engine.CharacterMovementComponent|SetGravityScale (Variables|/Script/Engine.Character|GetCharacterMovement _ascharacter) (Variables|Default|GetGravity%20Scale))
  (Variables|/Script/Engine.CharacterMovementComponent|SetAirControl (Variables|/Script/Engine.Character|GetCharacterMovement _ascharacter) (Variables|Default|GetAir%20Control))
  (Variables|/Script/Engine.MovementComponent|SetVelocity (Variables|/Script/Engine.Character|GetCharacterMovement _ascharacter) (Math|Vector|MakeVector (.x (Variables|/Script/Engine.MovementComponent|GetVelocity (Variables|/Script/Engine.Character|GetCharacterMovement _ascharacter))) (.y (Variables|/Script/Engine.MovementComponent|GetVelocity (Variables|/Script/Engine.Character|GetCharacterMovement _ascharacter))) 0.0))
  (Ability|Tasks|WaitInputRelease false
    (:OnRelease
      (Ability|EndAbility))))

(event Ability|EventOnEndAbility
  (params (bWasCancelled :type Boolean))
  (Variables|/Script/Engine.CharacterMovementComponent|SetGravityScale (Variables|/Script/Engine.Character|GetCharacterMovement (stale Ability|EventActivateAbility _ascharacter)) (Variables|Default|GetOriginal%20Gravity%20Scale))
  (Variables|/Script/Engine.CharacterMovementComponent|SetAirControl (Variables|/Script/Engine.Character|GetCharacterMovement (stale Ability|EventActivateAbility _ascharacter)) (Variables|Default|GetOriginal%20Air%20Control)))