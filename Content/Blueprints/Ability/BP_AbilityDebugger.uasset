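; BP_AbilityDebugger is an interactable debug actor for granting or removing player abilities through the Ability System Component.
; On interact, it either clears all of player 0's abilities or replaces those bound to the AbilityEnum input ID with AbilityClass, depending on ClearAbilities, and prints the result.
; The InRange and OutRange events move and reshape Cube3 as proximity feedback.
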(event EventBeginPlay)

(event Collision|EventActorBeginOverlap
  (params (OtherActor :type Actor%20Object%20Reference)))

(event EventInteractwith
  (bind _abilityenum (Variables|Default|GetAbilityEnum))
  (bind _returnvalue (Math|Conversions|ToInteger(Byte) _abilityenum))
  (bind _output_get (Variables|Default|SetAbilityComponent (Ability|GetAbilitySystemComponent (Game|GetPlayerCharacter 0))))
  (Utilities|IsValid _output_get
    (:Is%20Valid
      (if (Variables|Default|GetbClearAbilities)
        (Class|AbilitySystemComponent|ClearAllAbilities (Variables|Default|GetAbilityComponent))
        (Development|PrintString "All Abilities Removed")
        (else
          (Class|AbilitySystemComponent|ClearAllAbilitieswithInputID (Variables|Default|GetAbilityComponent) _returnvalue)
          (GameplayAbilities|GiveAbility (Variables|Default|GetAbilityComponent) (Variables|Default|GetAbility%20Class) 0 _returnvalue)
          (Development|PrintString (Utilities|String|Append (Utilities|String|EnumtoString _abilityenum) " Obtained")))))))

(event EventOutRange
  (bind _cube3 (Variables|Default|GetCube3))
  (Transformation|SetRelativeLocation _cube3 "50.000000,0.000000,10.000000" false false)
  (Transformation|SetRelativeScale3D _cube3 "0.100000,0.500000,0.100000"))

(event EventInRange
  (bind _cube3 (Variables|Default|GetCube3))
  (Transformation|SetRelativeLocation _cube3 "50.000000,0.000000,-10.000000" false false)
  (Transformation|SetRelativeScale3D _cube3 "0.100000,0.250000,0.500000"))

(fn ConstructionScript)