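; Gameplay ability for a charged dash: hold the input, then release to launch the character, with too short a hold cancelling.
; Clamped hold time feeds a logarithmic curve for dash strength.
; Direction follows the walkable floor's slope via right vector cross impact normal, or actor forward otherwise.
; A constant-force root motion task moves the character, keeps its velocity on finish, then ends the ability and forces the cooldown.
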(event Ability|EventActivateAbility
  (bind _ascharacter (Utilities|Casting|CastToCharacter (Ability|GetAvatarActorfromActorInfo)))
  (Variables|Default|SetCharacter _ascharacter)
  (bind _timeheld (Ability|Tasks|WaitInputRelease false)
    (:OnRelease
      (if (< _timeheld (Variables|Default|GetMinChargeTime))
        (Ability|EndAbility)
        (else
          (bind _dashnormal (CallFunction|DashVectorCalc))
          (bind _dashpower (CallFunction|DashPowerCalc _timeheld))
          (Ability|Tasks|ApplyRootMotionConstantForce "None" _dashnormal _dashpower 0.0 false 0 "MaintainLastRootMotionVelocity"
            (:OnFinish
              (Ability|EndAbility)
              (Ability|CommitAbilityCooldown false true))))))))

(fn DashPowerCalc
  (params (HoldTime :type Float%20%28double-precision%29))
  (return (* (Math|Float|Log (+ (Math|Float|Clamp(Float) HoldTime (Variables|Default|GetMinChargeTime) (Variables|Default|GetMaxChargeTime)) 1.0) 2.0) (Variables|Default|GetDashMultiplier))))

(fn DashVectorCalc
  (bind _character (Variables|Default|GetCharacter))
  (bind _character_2 (Variables|Default|GetCharacter))
  (bind _charactermovement (Variables|/Script/Engine.Character|GetCharacterMovement _character))
  (bind _currentfloor (Variables|/Script/Engine.CharacterMovementComponent|GetCurrentFloor _charactermovement))
  (bind (_bblockinghit _bwalkablefloor _blinetrace _floordist _linedist _hitresult) (Utilities|Struct|BreakFindFloorResult _currentfloor))
  (if _bwalkablefloor
    (return (Math|Vector|CrossProduct (Transformation|GetActorRightVector _character_2) (.ImpactNormal (Collision|BreakHitResult _hitresult))))
    (else
      (return (Transformation|GetActorForwardVector _character_2)))))