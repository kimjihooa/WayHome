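; BP_SaveDebugger is a debug actor in the Save folder that tests range response and dialogue option callbacks; it contains no save logic.
; InRange and OutRange lower and raise its Cube by setting relative location.
; From BeginPlay, it chains bindings from dialogue start to option creation, then binds the first two option buttons to Yes and No, which only print placeholder strings.
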(event Custom|BindOptions
  (EventDispatchers|BindEventtoOnOptionCreated (Variables|Default|GetDialogueWidget) (delegate Custom|Options)))

(event Custom|Options
  (for (_array_element _array_index) (Variables|/Game/Blueprints/Dialogue/WB_Dialogue.WB_Dialogue_C|GetOption%20Button (Variables|Default|GetDialogueWidget))
    (switch int _array_index
      (:0
        (EventDispatchers|BindEventtoOnClicked _array_element (delegate Custom|Yes)))
      (:1
        (EventDispatchers|BindEventtoOnClicked _array_element (delegate Custom|No))))))

(event Custom|Yes
  (Development|PrintString "oo"))

(event Custom|No
  (Development|PrintString "xx"))

(event EventBeginPlay
  (|CallParentFunction)
  (EventDispatchers|BindEventtoOnDialogueStarted (delegate Custom|BindOptions)))

(event EventOutRange
  (Transformation|SetRelativeLocation (Variables|Default|GetCube) "0.000000,50.000000,30.000000" false false))

(event EventInRange
  (Transformation|SetRelativeLocation (Variables|Default|GetCube) "0.000000,50.000000,-40.000000" false false))

(fn ConstructionScript
  (|CallParentFunction))