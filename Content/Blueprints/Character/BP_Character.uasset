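; Player character Blueprint with Gameplay Ability System abilities, save/load, swimming and a minimap toggle that also shows or hides checkpoint icons.
; Abilities are captured by input ID, stored in the save game or, on Destroyed, the GameInstance, then re-granted using array index as input ID.
; The GameInstance's LoadPlayerLocation flag selects save-driven restoration or level-transition restoration.
; Swimming toggles the physics volume's water flag and enables ascend input; Tick prints walk speed.
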(event Custom|StartSwimming
  (bind _charactermovement (Variables|Character|GetCharacterMovement))
  ;[1 1 1] Swimming
  (Variables|/Script/Engine.PhysicsVolume|SetbWaterVolume (Class|MovementComponent|GetPhysicsVolume _charactermovement) true)
  (Pawn|Components|CharacterMovement|SetMovementMode _charactermovement "MOVE_Swimming" 0))

(event Custom|StopSwimming
  (bind _charactermovement (Variables|Character|GetCharacterMovement))
  ;[1 1 1] Swimming
  (Variables|/Script/Engine.PhysicsVolume|SetbWaterVolume (Class|MovementComponent|GetPhysicsVolume _charactermovement) false)
  (Pawn|Components|CharacterMovement|SetMovementMode _charactermovement "MOVE_Walking" 0))

(event Input|EnhancedActionEvents|EnhancedInputActionIA_UIToggle
  (params (ActionValue :type Boolean) (ElapsedSeconds :type Float%20%28double-precision%29) (TriggeredSeconds :type Float%20%28double-precision%29) (InputAction :type Input%20Action%20Object%20Reference :default "/Game/Blueprints/Character/Input/IA_UIToggle.IA_UIToggle"))
  ;[0.7711 1 0.642] UI Toggle
  (:Started
    (bind _asbp_player_controller (Utilities|Casting|CastToBP_PlayerController (Game|GetPlayerController 0)))
    (if (== (Widget|GetVisibility (Variables|/Game/Blueprints/BP_PlayerController.BP_PlayerController_C|GetMinimapWidget _asbp_player_controller)) 0)
      (Widget|SetVisibility (Variables|/Game/Blueprints/BP_PlayerController.BP_PlayerController_C|GetMinimapWidget _asbp_player_controller) "Hidden")
      (bind _outactors (Actor|GetAllActorswithInterface "/Game/Blueprints/Map/BPI_MapCheckpoint.BPI_MapCheckpoint_C"))
      (for _array_element _outactors
        (Class|BPIMapCheckpoint|HideIcon(Message) _array_element))
      (else
        (Widget|SetVisibility (Variables|/Game/Blueprints/BP_PlayerController.BP_PlayerController_C|GetMinimapWidget _asbp_player_controller) "Visible")
        (bind _outactors_2 (Actor|GetAllActorswithInterface "/Game/Blueprints/Map/BPI_MapCheckpoint.BPI_MapCheckpoint_C"))
        (for _array_element_2 _outactors_2
          (Class|BPIMapCheckpoint|ShowIcon(Message) _array_element_2))))))

(event Input|EnhancedActionEvents|EnhancedInputActionIA_Ascend
  (params (ActionValue :type Float%20%28double-precision%29) (ElapsedSeconds :type Float%20%28double-precision%29) (TriggeredSeconds :type Float%20%28double-precision%29) (InputAction :type Input%20Action%20Object%20Reference :default "/Game/Blueprints/Character/Input/IA_Ascend.IA_Ascend"))
  (if (== (Variables|/Script/Engine.CharacterMovementComponent|GetMovementMode (Variables|Character|GetCharacterMovement)) 4)
    (Pawn|Input|AddMovementInput "0.000000,0.000000,1.000000" (* ActionValue 1.0) false)))

(event EventBeginPlay
  (|CallParentFunction)
  (bind _asbp_game_instance (Utilities|Casting|CastToBP_GameInstance (Game|GetGameInstance)))
  (if (Variables|/Game/Blueprints/Save/BP_GameInstance.BP_GameInstance_C|GetbLoadPlayerLocation _asbp_game_instance)
    ;[1 1 1] On First Load
    (Class|BPIPersistence|RequsetLoad(Message) (Game|GetGameInstance) self)
    (else
      ;[1 1 1] On Level Load
      (for (_array_element _array_index) (Variables|/Game/Blueprints/Save/BP_GameInstance.BP_GameInstance_C|GetAbilityList _asbp_game_instance)
        (if (Utilities|IsValidClass _array_element)
          (GameplayAbilities|GiveAbility (Variables|Default|GetAbilitySystemComponent) _array_element 0 _array_index))))))

(event EventDestroyed
  (bind _asbp_game_instance (Utilities|Casting|CastToBP_GameInstance (Game|GetGameInstance)))
  (bind _abilities (CallFunction|GetAbilitiesList))
  (Variables|/Game/Blueprints/Save/BP_GameInstance.BP_GameInstance_C|SetAbilityList _asbp_game_instance _abilities))

(event EventLoadData
  (params (SaveGame :type BP%20Save%20Game%20Object%20Reference))
  ;[1 0.5932 0.8631] Save & Load
  ;;[0.6685 0.7584 1] Load Transform
  (bind _asbp_game_instance (Utilities|Casting|CastToBP_GameInstance (Game|GetGameInstance)))
  (if (Variables|/Game/Blueprints/Save/BP_GameInstance.BP_GameInstance_C|GetbLoadPlayerLocation _asbp_game_instance)
    (Transformation|SetActorLocation (Variables|/Game/Blueprints/Save/BP_SaveGame.BP_SaveGame_C|GetPlayerLocation SaveGame) false false)
    (Transformation|SetActorRotation (Variables|/Game/Blueprints/Save/BP_SaveGame.BP_SaveGame_C|GetPlayerRotation SaveGame))
    (Variables|/Game/Blueprints/Save/BP_GameInstance.BP_GameInstance_C|SetbLoadPlayerLocation _asbp_game_instance false))
  ;;[0.801 0.8437 1] Load Ability
  (for (_array_element _array_index) (Variables|/Game/Blueprints/Save/BP_SaveGame.BP_SaveGame_C|GetAbilities SaveGame)
    (if (Utilities|IsValidClass _array_element)
      (GameplayAbilities|GiveAbility (Variables|Default|GetAbilitySystemComponent) _array_element 0 _array_index))))

(event EventSaveData
  (params (SaveGame :type BP%20Save%20Game%20Object%20Reference))
  ;[1 0.5932 0.8631] Save & Load
  ;;[1 0.4366 0.4665] Save Transform
  (bind _returnvalue (Game|GetCurrentLevelName true))
  (Variables|/Game/Blueprints/Save/BP_SaveGame.BP_SaveGame_C|SetPlayerLevel SaveGame _returnvalue)
  (Variables|/Game/Blueprints/Save/BP_SaveGame.BP_SaveGame_C|SetPlayerLocation SaveGame (Transformation|GetActorLocation))
  (Variables|/Game/Blueprints/Save/BP_SaveGame.BP_SaveGame_C|SetPlayerRotation SaveGame (Transformation|GetActorRotation))
  ;;[1 0.6036 0.6235] Ability
  (bind _abilities (CallFunction|GetAbilitiesList))
  (Variables|/Game/Blueprints/Save/BP_SaveGame.BP_SaveGame_C|SetAbilities SaveGame _abilities))

(event EventTick
  (params (DeltaSeconds :type Float%20%28single-precision%29))
  (Development|PrintString (Utilities|String|ToString(Float) (Variables|/Script/Engine.CharacterMovementComponent|GetMaxWalkSpeed (Variables|Character|GetCharacterMovement)))))

(fn ConstructionScript)

(fn GetAbilitiesList
  (bind _abilitylist (LocalVariables|GetAbilityList))
  (LocalVariables|SetLoop 0)
  (bind _output_get (LocalVariables|SetLoopLength (|GetNumEnumEntries)))
  (if (> _output_get (LocalVariables|GetLoop)) :!label _label
    (bind _outabilityhandles (Class|AbilitySystemComponent|FindAllAbilitieswithInputID (Variables|Default|GetAbilitySystemComponent) (LocalVariables|GetLoop)))
    (if (Utilities|Array|IsEmpty _outabilityhandles)
      (Utilities|Array|Add _abilitylist 0)
      (else
        (Utilities|Array|Add _abilitylist (Utilities|GetClass (.ReturnValue (Ability|GameplayAbility|GetGameplayAbilityfromSpecHandle (Variables|Default|GetAbilitySystemComponent) (Utilities|Array|Get(acopy) _outabilityhandles)))))))
    (LocalVariables|SetLoop (+ (LocalVariables|GetLoop) 1))
    (goto _label)
    (else
      (return (LocalVariables|GetAbilityList)))))