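; BP_Flower is a plant that grows upward while in BP_Water, lowering the water's RaiseNum as it drinks.
; An upward trace at BeginPlay sets the height limit.
; Box overlap resumes paused looping timers that lift GrowPoint and attach cylinder stem segments at a speed-scaled interval.
; Box exit or Flower overlap with water restores the drain and pauses growth, while destruction also restores the drain.
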(event OnComponentBeginOverlap(Box)
  (params (OverlappedComponent :type Primitive%20Component%20Object%20Reference) (OtherActor :type Actor%20Object%20Reference) (OtherComp :type Primitive%20Component%20Object%20Reference) (OtherBodyIndex :type Integer) (bFromSweep :type Boolean) (SweepResult :type Hit%20Result%20Structure%20%28by%20ref%29))
  (bind _asbp_water (Utilities|Casting|CastToBP_Water OtherActor))
  (Variables|Default|SetWater _asbp_water)
  (Variables|/Game/Blueprints/Swim/BP_Water.BP_Water_C|SetRaiseNum _asbp_water (- (Variables|/Game/Blueprints/Swim/BP_Water.BP_Water_C|GetRaiseNum _asbp_water) (Variables|Default|GetDrainNum)))
  (CallFunction|StartGrowing))

(event OnComponentEndOverlap(Box)
  (params (OverlappedComponent :type Primitive%20Component%20Object%20Reference) (OtherActor :type Actor%20Object%20Reference) (OtherComp :type Primitive%20Component%20Object%20Reference) (OtherBodyIndex :type Integer))
  (bind _asbp_water (Utilities|Casting|CastToBP_Water (stale OnComponentBeginOverlap(Flower) OtherActor)))
  (Variables|/Game/Blueprints/Swim/BP_Water.BP_Water_C|SetRaiseNum _asbp_water (+ (Variables|/Game/Blueprints/Swim/BP_Water.BP_Water_C|GetRaiseNum _asbp_water) (Variables|Default|GetDrainNum)))
  (CallFunction|StopGrowing))

(event OnComponentBeginOverlap(Flower)
  (params (OverlappedComponent :type Primitive%20Component%20Object%20Reference) (OtherActor :type Actor%20Object%20Reference) (OtherComp :type Primitive%20Component%20Object%20Reference) (OtherBodyIndex :type Integer) (bFromSweep :type Boolean) (SweepResult :type Hit%20Result%20Structure%20%28by%20ref%29))
  (bind _asbp_water (Utilities|Casting|CastToBP_Water OtherActor))
  (Variables|/Game/Blueprints/Swim/BP_Water.BP_Water_C|SetRaiseNum _asbp_water (+ (Variables|/Game/Blueprints/Swim/BP_Water.BP_Water_C|GetRaiseNum _asbp_water) (Variables|Default|GetDrainNum)))
  (CallFunction|StopGrowing))

(event Custom|SpawnStem
  (bind _returnvalue (Game|AddComponentbyClass "/Script/Engine.StaticMeshComponent" false))
  (Transformation|AttachComponentToComponent _returnvalue (Variables|Default|GetGrowPoint) "None" "KeepWorld" "KeepRelative" "KeepRelative" true)
  (Components|StaticMesh|SetStaticMesh _returnvalue "/Engine/BasicShapes/Cylinder.Cylinder")
  (Variables|/Script/Engine.PrimitiveComponent|SetbGenerateOverlapEvents _returnvalue false)
  (Collision|SetCollisionProfileName _returnvalue "IgnoreOnlyVisibility" false :!class /Script/Engine.PrimitiveComponent))

(event Custom|Grow
  (if (< (.z (Transformation|GetWorldLocation (Variables|Default|GetGrowPoint))) (- (Variables|Default|GetGrowLimit) (Variables|Default|GetGrowLimitOffset)))
    (Transformation|AddWorldOffset (Variables|Default|GetGrowPoint) (Math|Vector|MakeVector 0.0 0.0 (Variables|Default|GetGrowSpeed)) false false)
    (else
      (Utilities|Time|ClearandInvalidateTimerbyHandle (Variables|Default|GetStemTimer))
      (Utilities|Time|ClearandInvalidateTimerbyHandle (Variables|Default|GetGrowTimer)))))

(event Custom|StartGrowing
  (if (not (Variables|Default|GetbIsGrowing))
    (Variables|Default|SetbIsGrowing true)
    (Utilities|Time|UnpauseTimerbyHandle (Variables|Default|GetGrowTimer))
    (Utilities|Time|UnpauseTimerbyHandle (Variables|Default|GetStemTimer))))

(event Custom|StopGrowing
  (if (Variables|Default|GetbIsGrowing)
    (Variables|Default|SetbIsGrowing false)
    (Utilities|Time|PauseTimerbyHandle (Variables|Default|GetGrowTimer))
    (Utilities|Time|PauseTimerbyHandle (Variables|Default|GetStemTimer))))

(event EventBeginPlay
  (bind _returnvalue (Transformation|GetActorLocation))
  (Utilities|FlowControl|Sequence
    (:then_0
      (bind _outhit (Collision|LineTraceByChannel _returnvalue (+ _returnvalue "0.000000,0.000000,10000.000000") "TraceTypeQuery1" false 0 "None"))
      (Variables|Default|SetGrowLimit (.Z (Math|Vector|BreakVector (.Location (Collision|BreakHitResult _outhit))))))
    (:then_1
      (CallFunction|SpawnStem)
      (bind _returnvalue_2 (Utilities|Time|SetTimerbyEvent (delegate Custom|Grow) 0.01 true))
      (bind _output_get (Variables|Default|SetGrowTimer _returnvalue_2))
      (Utilities|Time|PauseTimerbyHandle _output_get)
      (bind _returnvalue_3 (Utilities|Time|SetTimerbyEvent (delegate Custom|SpawnStem) (/ 1e+02 (* (Variables|Default|GetGrowSpeed) 1e+02)) true))
      (bind _output_get_2 (Variables|Default|SetStemTimer _returnvalue_3))
      (Utilities|Time|PauseTimerbyHandle _output_get_2))))

(event EventDestroyed
  (bind _water (Variables|Default|GetWater))
  (Utilities|IsValid _water
    (:Is%20Valid
      (Variables|/Game/Blueprints/Swim/BP_Water.BP_Water_C|SetRaiseNum _water (+ (Variables|/Game/Blueprints/Swim/BP_Water.BP_Water_C|GetRaiseNum _water) (Variables|Default|GetDrainNum))))))

(fn ConstructionScript)