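; BP_BigRoot is a root obstacle that drains water and can be smashed by a fast-moving character.
; While its Cone overlaps a BP_Water, it lowers that water's RaiseNum by DrainNum and adds it back when the overlap ends.
; A hit on the Cone from BP_Character destroys the root if the character's movement speed is at least ImpactLimit.
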(event OnComponentBeginOverlap(Cone)
  (params (OverlappedComponent :type Primitive%20Component%20Object%20Reference) (OtherActor :type Actor%20Object%20Reference) (OtherComp :type Primitive%20Component%20Object%20Reference) (OtherBodyIndex :type Integer) (bFromSweep :type Boolean) (SweepResult :type Hit%20Result%20Structure%20%28by%20ref%29))
  (bind _asbp_water (Utilities|Casting|CastToBP_Water OtherActor))
  (Variables|/Game/Blueprints/Swim/BP_Water.BP_Water_C|SetRaiseNum _asbp_water (- (Variables|/Game/Blueprints/Swim/BP_Water.BP_Water_C|GetRaiseNum _asbp_water) (Variables|Default|GetDrainNum))))

(event OnComponentEndOverlap(Cone)
  (params (OverlappedComponent :type Primitive%20Component%20Object%20Reference) (OtherActor :type Actor%20Object%20Reference) (OtherComp :type Primitive%20Component%20Object%20Reference) (OtherBodyIndex :type Integer))
  (bind _asbp_water (Utilities|Casting|CastToBP_Water OtherActor))
  (Variables|/Game/Blueprints/Swim/BP_Water.BP_Water_C|SetRaiseNum _asbp_water (+ (Variables|/Game/Blueprints/Swim/BP_Water.BP_Water_C|GetRaiseNum _asbp_water) (Variables|Default|GetDrainNum))))

(event OnComponentHit(Cone)
  (params (HitComponent :type Primitive%20Component%20Object%20Reference) (OtherActor :type Actor%20Object%20Reference) (OtherComp :type Primitive%20Component%20Object%20Reference) (NormalImpulse :type Vector :default "0, 0, 0") (Hit :type Hit%20Result%20Structure%20%28by%20ref%29))
  (bind _asbp_character (Utilities|Casting|CastToBP_Character OtherActor))
  (if (>= (Math|Vector|VectorLength (Variables|/Script/Engine.MovementComponent|GetVelocity (Variables|/Script/Engine.Character|GetCharacterMovement _asbp_character))) (Variables|Default|GetImpactLimit))
    (Actor|DestroyActor)))

(event EventBeginPlay)

(event Collision|EventActorBeginOverlap
  (params (OtherActor :type Actor%20Object%20Reference)))

(event EventTick
  (params (DeltaSeconds :type Float%20%28single-precision%29)))

(fn ConstructionScript)