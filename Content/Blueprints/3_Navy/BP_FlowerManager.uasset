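; Manager actor that lets the player pick up and place flowers through the character's gimmick interact event, tracking the count in a flower HUD widget.
; A capsule trace ahead of the player, ignoring water, collects ground or floating flowers up to a small cap.
; Otherwise it spends a flower, spawning a floating one when the water's swim mode qualifies, or a ground one where a downward trace hits.
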(event Custom|FlowerToggle
  (bind _returnvalue (Game|GetPlayerCharacter 0))
  (bind _returnvalue_2 (Game|GetPlayerCharacter 0))
  (bind _returnvalue_3 (Game|GetPlayerCharacter 0))
  (bind _bowpdistance (Variables|Default|GetBowpDistance))
  (bind _bowpdistance_2 (Variables|Default|GetBowpDistance))
  (bind _returnvalue_4 (Transformation|GetActorForwardVector _returnvalue_3))
  (bind _returnvalue_5 (Transformation|GetActorForwardVector _returnvalue_2))
  (bind _returnvalue_6 (Transformation|GetActorLocation _returnvalue_2))
  (bind _returnvalue_7 (Transformation|GetActorForwardVector _returnvalue))
  (bind _returnvalue_8 (Transformation|GetActorLocation _returnvalue))
  (bind _returnvalue_9 (* _returnvalue_7 _bowpdistance_2))
  (bind _returnvalue_10 (* _bowpdistance _returnvalue_5))
  (bind _returnvalue_11 (+ _returnvalue_8 _returnvalue_9))
  (bind _returnvalue_12 (+ _returnvalue_6 _returnvalue_10))
  (bind _outhit (Collision|CapsuleTraceByChannel _returnvalue_11 _returnvalue_11 (Variables|Default|GetBowpRadious) 1.2e+02 "TraceTypeQuery3" false (Variables|Default|GetIgnoreActors) "ForDuration"))
  (bind _asbp_flower (Utilities|Casting|CastToBP_Flower (.HitActor (Collision|BreakHitResult _outhit)))
    (:then
      (if (<= (Variables|Default|GetFlowerNum) 4)
        (Actor|DestroyActor _asbp_flower)
        (Default|AddFlower (Variables|Default|GetFlowerWidget) (Variables|Default|GetFlowerNum))
        (Math|Integer|IncrementInt (Variables|Default|GetFlowerNum))))
    (:CastFailed
      (bind _asbp_floating_flower (Utilities|Casting|CastToBP_FloatingFlower (.HitActor (Collision|BreakHitResult _outhit)))
        (:then
          (if (<= (Variables|Default|GetFlowerNum) 4)
            (Actor|DestroyActor _asbp_floating_flower)
            (Default|AddFlower (Variables|Default|GetFlowerWidget) (Variables|Default|GetFlowerNum))
            (Math|Integer|IncrementInt (Variables|Default|GetFlowerNum))))
        (:CastFailed
          ;[1 1 1] Spawn Floating Flower
          (if (>= (Variables|/Game/Blueprints/Swim/BP_Water.BP_Water_C|GetSwimMode (Variables|Default|GetWaterActor)) 2)
            (if (> (Variables|Default|GetFlowerNum) 0)
              (Game|SpawnActorfromClass "/Game/Blueprints/3_Navy/BP_FloatingFlower.BP_FloatingFlower_C" (Math|Transform|MakeTransform (+ (Transformation|GetActorLocation _returnvalue_3) (* (Variables|Default|GetBowpDistance) _returnvalue_4)) (Math|Conversions|RotationFromXVector _returnvalue_4) "1.000000,1.000000,1.000000") "Undefined" "MultiplyWithRoot" 0 0)
              (Math|Integer|DecrementInt (Variables|Default|GetFlowerNum)
                (:%20%20
                  (Default|RemoveFlower (Variables|Default|GetFlowerWidget) (Variables|Default|GetFlowerNum)))))
            (elif (> (Variables|Default|GetFlowerNum) 0)
              (bind _returnvalue_13 (Collision|LineTraceByChannel _returnvalue_12 (- _returnvalue_12 "0.000000,0.000000,200.000000") "TraceTypeQuery1" false 0 "ForDuration"))
              (if _returnvalue_13
                (Game|SpawnActorfromClass "/Game/Blueprints/3_Navy/BP_Flower.BP_Flower_C" (Math|Transform|MakeTransform (- _returnvalue_12 "0.000000,0.000000,75.000000") (Math|Conversions|RotationFromXVector _returnvalue_5) "1.000000,1.000000,1.000000") "Undefined" "MultiplyWithRoot" 0 0)
                (Math|Integer|DecrementInt (Variables|Default|GetFlowerNum)
                  (:%20%20
                    (Default|RemoveFlower (Variables|Default|GetFlowerWidget) (Variables|Default|GetFlowerNum))))))))))))

(event EventBeginPlay
  (bind _asbp_character (Utilities|Casting|CastToBP_Character (Game|GetPlayerCharacter 0)))
  (EventDispatchers|BindEventtoOnGimmikInteract _asbp_character (delegate Custom|FlowerToggle))
  (bind _returnvalue (UserInterface|CreateWidget "/Game/Blueprints/3_Navy/WB_Flower.WB_Flower_C"))
  (bind _output_get (Variables|Default|SetFlowerWidget _returnvalue))
  (UserInterface|Viewport|AddtoViewport _output_get 0)
  (bind _asbp_player_controller (Utilities|Casting|CastToBP_PlayerController (Game|GetPlayerController 0)))
  (Utilities|Array|Add (Variables|/Game/Blueprints/BP_PlayerController.BP_PlayerController_C|GetOtherWidgets _asbp_player_controller) _output_get)
  (bind _outactors (Actor|GetAllActorsOfClass "/Game/Blueprints/Swim/BP_Water.BP_Water_C"))
  (bind _output_get_2 (Variables|Default|SetIgnoreActors _outactors))
  (Utilities|Array|Add _output_get_2 (Game|GetPlayerCharacter 0)))

(event EventDestroyed
  (bind _asbp_character (Utilities|Casting|CastToBP_Character (Game|GetPlayerCharacter 0)))
  (EventDispatchers|UnbindEventfromOnGimmikInteract _asbp_character (delegate Custom|FlowerToggle))
  (bind _asbp_player_controller (Utilities|Casting|CastToBP_PlayerController (Game|GetPlayerController 0)))
  (Utilities|Array|RemoveItem (Variables|/Game/Blueprints/BP_PlayerController.BP_PlayerController_C|GetOtherWidgets _asbp_player_controller) (Variables|Default|GetFlowerWidget)))

(fn ConstructionScript)