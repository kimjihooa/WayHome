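; Player controller that creates and manages the gameplay HUD widgets.
; On BeginPlay it adds the minimap and a hidden pause popup to the viewport, then calls OnAllWidgetCreated.
; ToggleHideAllWidgets uses minimap visibility as the state to show or hide the minimap, the OtherWidgets list and icons on map checkpoint actors, which it reaches through BPI_MapCheckpoint.
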(event EventBeginPlay
  (Utilities|FlowControl|Sequence
    (:then_0
      (bind _returnvalue (UserInterface|CreateWidget "/Game/Blueprints/Map/WB_MiniMap.WB_MiniMap_C"))
      (bind _output_get (Variables|Default|SetMinimapWidget _returnvalue))
      (UserInterface|Viewport|AddtoViewport _output_get 0))
    (:then_1
      (bind _returnvalue_2 (UserInterface|CreateWidget "/Game/UI/GamePlayPausepopup/WB_GamePlayPausePopUp.WB_GamePlayPausePopUp_C"))
      (bind _output_get_2 (Variables|Default|SetPauseWidget _returnvalue_2))
      (UserInterface|Viewport|AddtoViewport _output_get_2 0)
      (Variables|/Script/UMG.Widget|SetVisibility _output_get_2 "Hidden"))
    (:then_2
      (Default|CallOnAllWidgetCreated))))

(event EventTick
  (params (DeltaSeconds :type Float%20%28single-precision%29)))

(fn ConstructionScript)

(fn ToggleHideAllWidgets
  (bind _minimapwidget (Variables|Default|GetMinimapWidget))
  (bind _otherwidgets (Variables|Default|GetOtherWidgets))
  (if (== (Widget|GetVisibility _minimapwidget) 0)
    (Widget|SetVisibility _minimapwidget "Hidden")
    (bind _outactors (Actor|GetAllActorswithInterface "/Game/Blueprints/Map/BPI_MapCheckpoint.BPI_MapCheckpoint_C"))
    (for _array_element _outactors
      (Class|BPIMapCheckpoint|HideIcon(Message) _array_element))
    (for _array_element_2 _otherwidgets
      (Variables|/Script/UMG.Widget|SetVisibility _array_element_2 "Hidden"))
    (else
      (Widget|SetVisibility _minimapwidget "Visible")
      (bind _outactors_2 (Actor|GetAllActorswithInterface "/Game/Blueprints/Map/BPI_MapCheckpoint.BPI_MapCheckpoint_C"))
      (for _array_element_3 _outactors_2
        (Class|BPIMapCheckpoint|ShowIcon(Message) _array_element_3))
      (for _array_element_4 _otherwidgets
        (Variables|/Script/UMG.Widget|SetVisibility _array_element_4 "Visible")))))