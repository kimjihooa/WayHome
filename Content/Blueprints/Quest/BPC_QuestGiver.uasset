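; Quest giver component that lets its owner add quests and update their objectives through the level's quest manager.
; On BeginPlay it finds and caches the BP_QuestManager actor, printing an error if none exists.
; AddQuest looks up the quest ID in a data table and passes its textures and question flags to the manager.
; Half-clear and clear events forward quest and object indices straight to the manager.
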(event Custom|AddQuest
  (params (QuestID :type Name))
  (bind _questdatatable (Variables|Default|GetQuestDataTable))
  (bind _returnvalue (Utilities|GetDataTableRow _questdatatable QuestID)
    (:then
      (Default|AddQuest (Variables|Default|GetQuestManager) QuestID (.ObjectTextures (Utilities|Struct|BreakS_Quest _returnvalue)) (.bIsQuestion (Utilities|Struct|BreakS_Quest _returnvalue)) _questdatatable))
    (:RowNotFound
      (Development|PrintString "Quest Row Not Found"))))

(event Custom|HalfClearObject
  (params (QuestID :type Name) (ObjectIndex :type Integer))
  (Default|HalfClearObject (Variables|Default|GetQuestManager) QuestID ObjectIndex))

(event Custom|ClearObject
  (params (QuestID :type Name) (ObjectIndex :type Integer))
  (Default|ClearObject (Variables|Default|GetQuestManager) QuestID ObjectIndex))

(event EventBeginPlay
  (bind _returnvalue (Actor|GetActorOfClass "/Game/Blueprints/Quest/BP_QuestManager.BP_QuestManager_C"))
  (Utilities|IsValid _returnvalue
    (:Is%20Valid
      (Variables|Default|SetQuestManager _returnvalue))
    (:Is%20Not%20Valid
      (Development|PrintString "QuestManagerNotFound"))))