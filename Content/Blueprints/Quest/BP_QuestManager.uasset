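; Quest manager that tracks one active quest and its objectives, with a QuestID of "-1" meaning none is active.
; It creates a hidden WB_Quest widget on BeginPlay and forwards visibility, bubble-size and objective updates to it.
; AddQuest rejects a quest while one is active, otherwise storing its objects and question flags.
; ClearObject marks objectives done, and once all are, resets the quest and fires the OnQuestCleared dispatcher.
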(event Custom|AddQuest
  (params (QuestID :type Name) (QuestObjects :type Array%20of%20Soft%20Object%20Path%20Structures) (bQuestions :type Array%20of%20Booleans))
  (bind _bobjectclear (Variables|Default|GetbObjectClear))
  (if (or (== (Variables|Default|GetQuestID) QuestID) (!= (Variables|Default|GetQuestID) "-1"))
    (Development|PrintString (Utilities|String|Append (Utilities|String|MakeLiteralString "Already has Quest ") (Utilities|String|ToString(Name) (Variables|Default|GetQuestID))))
    (else
      (Variables|Default|SetQuestID QuestID)
      (Variables|Default|SetObjects QuestObjects)
      (Variables|Default|SetbQuestions bQuestions)
      (Default|AddObjects (Variables|Default|GetQuestWidget) QuestObjects bQuestions)
      (Utilities|Array|Resize _bobjectclear (Utilities|Array|Length bQuestions))
      (for (_ _array_index) _bobjectclear
        (Utilities|Array|SetArrayElem _bobjectclear _array_index false)))))

(event Custom|HalfClearObject
  (params (QuestID :type Name) (ObjectIndex :type Integer))
  (if (== QuestID (Variables|Default|GetQuestID))
    (Default|HalfClearObject (Variables|Default|GetQuestWidget) ObjectIndex)))

(event Custom|ClearObject
  (params (QuestID :type Name) (ObjectIndex :type Integer))
  (Default|ClearObject (Variables|Default|GetQuestWidget) ObjectIndex)
  (Utilities|Array|SetArrayElem (Variables|Default|GetbObjectClear) ObjectIndex true)
  (bind _bquestcleared (CallFunction|CheckQuestClear))
  (if _bquestcleared
    (CallFunction|ClearQuest)))

(event Custom|ShowUI
  (Widget|SetVisibility (Variables|Default|GetQuestWidget) "Visible"))

(event Custom|ClearQuest
  (if (!= (Variables|Default|GetQuestID) "-1")
    (Development|PrintString (Utilities|String|Append (Utilities|String|Append (Utilities|String|MakeLiteralString "Quest ") (Utilities|String|ToString(Name) (Variables|Default|GetQuestID))) " Cleared"))
    (Variables|Default|SetQuestID "-1")
    (Utilities|Array|Clear (Variables|Default|GetObjects))
    (Utilities|Array|Clear (Variables|Default|GetbQuestions))
    (Default|CallOnQuestCleared)))

(event Custom|HideUI
  (Widget|SetVisibility (Variables|Default|GetQuestWidget) "Hidden"))

(event Custom|ShowSmall
  (Default|ShowSmallBubble (Variables|Default|GetQuestWidget)))

(event Custom|ShowShrinked
  (Default|ShowShrinkedBubble (Variables|Default|GetQuestWidget)))

(event EventBeginPlay
  (bind _returnvalue (UserInterface|CreateWidget "/Game/Blueprints/Quest/WB_Quest.WB_Quest_C"))
  (bind _output_get (Variables|Default|SetQuestWidget _returnvalue))
  (UserInterface|Viewport|AddtoViewport _output_get 0)
  (Widget|SetVisibility _output_get "Hidden"))

(fn ConstructionScript)

(fn CheckQuestClear
  (for _array_element (Variables|Default|GetbObjectClear)
    (if (not _array_element)
      (return false)))
  (return true))