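; Checkpoint actor that shows a marker icon on the player's minimap.
; Shortly after BeginPlay it takes the minimap widget from BP_HUD and creates a checkpoint icon widget in the viewport.
; Tick feeds that widget the checkpoint's 2D offset from the player character.
; Wrapper events change the icon's texture, size and visibility, retrying once after a short delay if the widget is not yet valid.
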(event Custom|ChangeIconTexture
  (params (Texture :type Texture%202D%20Object%20Reference))
  (bind _minimapcheckpointwidget (Variables|Default|GetMinimapCheckpointWidget))
  ;[1 1 1] Custom Settings Wrapper
  (Utilities|IsValid _minimapcheckpointwidget
    (:Is%20Valid
      (Default|ChangeIcon _minimapcheckpointwidget Texture :!label _label))
    (:Is%20Not%20Valid
      (Utilities|FlowControl|Delay 0.2)
      (Utilities|IsValid (Variables|Default|GetMinimapCheckpointWidget)
        (:Is%20Valid
          (goto _label))
        (:Is%20Not%20Valid
          (Development|PrintString "Checkpoint Widget Not Valid"))))))

(event Custom|ChangeIconSize
  (params (InSize :type Vector%202D%20Structure))
  (bind _minimapcheckpointwidget (Variables|Default|GetMinimapCheckpointWidget))
  ;[1 1 1] Custom Settings Wrapper
  (Utilities|IsValid _minimapcheckpointwidget
    (:Is%20Valid
      (Default|ChangeSize _minimapcheckpointwidget InSize :!label _label))
    (:Is%20Not%20Valid
      (Utilities|FlowControl|Delay 0.2)
      (Utilities|IsValid (Variables|Default|GetMinimapCheckpointWidget)
        (:Is%20Valid
          (goto _label))
        (:Is%20Not%20Valid
          (Development|PrintString "Checkpoint Widget Not Valid"))))))

(event Custom|HideIcon
  (bind _minimapcheckpointwidget (Variables|Default|GetMinimapCheckpointWidget))
  ;[1 1 1] Custom Settings Wrapper
  (Utilities|IsValid _minimapcheckpointwidget
    (:Is%20Valid
      (Default|HideIcon _minimapcheckpointwidget :!label _label))
    (:Is%20Not%20Valid
      (Utilities|FlowControl|Delay 0.2)
      (Utilities|IsValid (Variables|Default|GetMinimapCheckpointWidget)
        (:Is%20Valid
          (goto _label))
        (:Is%20Not%20Valid
          (Development|PrintString "Checkpoint Widget Not Valid"))))))

(event Custom|ShowIcon
  (bind _minimapcheckpointwidget (Variables|Default|GetMinimapCheckpointWidget))
  ;[1 1 1] Custom Settings Wrapper
  (Utilities|IsValid _minimapcheckpointwidget
    (:Is%20Valid
      (Default|ShowIcon _minimapcheckpointwidget :!label _label))
    (:Is%20Not%20Valid
      (Utilities|FlowControl|Delay 0.2)
      (Utilities|IsValid (Variables|Default|GetMinimapCheckpointWidget)
        (:Is%20Valid
          (goto _label))
        (:Is%20Not%20Valid
          (Development|PrintString "Checkpoint Widget Not Valid"))))))

(event EventBeginPlay
  (Utilities|FlowControl|Delay 0.1)
  (bind _asbp_hud (Utilities|Casting|CastToBP_HUD (HUD|GetHUD (Game|GetPlayerController 0))))
  (Utilities|IsValid (Variables|/Game/Blueprints/BP_HUD.BP_HUD_C|GetMinimapWidget _asbp_hud)
    (:Is%20Valid
      (Variables|Default|SetMinimapWidget (Variables|/Game/Blueprints/BP_HUD.BP_HUD_C|GetMinimapWidget _asbp_hud))
      (bind _returnvalue (UserInterface|CreateWidget "/Game/Blueprints/Map/WB_MiniMapCheckpoint.WB_MiniMapCheckpoint_C" 0 (Variables|/Game/Blueprints/BP_HUD.BP_HUD_C|GetMinimapWidget _asbp_hud) (Variables|Default|GetbShowIconOutside)))
      (bind _output_get (Variables|Default|SetMinimapCheckpointWidget _returnvalue))
      (UserInterface|Viewport|AddtoViewport _output_get 0))))

(event EventTick
  (params (DeltaSeconds :type Float%20%28single-precision%29))
  (bind _minimapcheckpointwidget (Variables|Default|GetMinimapCheckpointWidget))
  ;[0.434 0.9402 1] Update Position
  (Utilities|IsValid _minimapcheckpointwidget
    (:Is%20Valid
      (Default|UpdateIconLocation _minimapcheckpointwidget (Math|Conversions|ToVector2D(Vector) (- (Transformation|GetActorLocation) (Transformation|GetActorLocation (Game|GetPlayerCharacter 0))))))))

(fn ConstructionScript)