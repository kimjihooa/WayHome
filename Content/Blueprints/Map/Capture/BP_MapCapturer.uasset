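; BP_MapCapturer renders an orthographic top-down-style snapshot of the level and saves it as a PNG, likely for map imagery.
; On BeginPlay it configures its SceneCaptureComponent2D with a set ortho width and LDR final color, then captures once into RT_MapCapture.
; After a short delay it exports the render target to the project's Saved folder under FileName and prints the path and success result.
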(event Custom|OnComplete
  (params (bSuccess :type Boolean))
  (Development|PrintString (Utilities|String|ToString(Boolean) bSuccess)))

(event EventBeginPlay
  (bind _returnvalue (Class|KismetSystemLibrary|GetProjectDirectory))
  (bind _scenecapturecomponent2d (Variables|Default|GetSceneCaptureComponent2D))
  (bind _filename (Variables|Default|GetFileName))
  (bind _returnvalue_2 (Utilities|String|Append _returnvalue "Saved/"))
  (bind _returnvalue_3 (Utilities|String|Append _returnvalue_2 _filename))
  (bind _returnvalue_4 (Utilities|String|Append _returnvalue_3 ".PNG"))
  (Variables|/Script/Engine.SceneCaptureComponent2D|SetProjectionType _scenecapturecomponent2d "Orthographic")
  (Variables|/Script/Engine.SceneCaptureComponent2D|SetOrthoWidth _scenecapturecomponent2d (Variables|Default|GetOrtho%20Width))
  (Variables|/Script/Engine.SceneCaptureComponent|SetCaptureSource _scenecapturecomponent2d "SCS_FinalColorLDR")
  (bind _output_get (Variables|/Script/Engine.SceneCaptureComponent2D|SetTextureTarget _scenecapturecomponent2d "/Game/Blueprints/Map/Capture/RT_MapCapture.RT_MapCapture"))
  (bind _output_get_2 (Variables|Default|SetRenderTarget _output_get))
  (Variables|/Script/Engine.SceneCaptureComponent|SetbCaptureEveryFrame _scenecapturecomponent2d false)
  (Rendering|SceneCapture|CaptureScene _scenecapturecomponent2d :!class /Script/Engine.SceneCaptureComponent2D)
  (Utilities|FlowControl|Delay 1.0)
  (Development|PrintString _returnvalue_4 true true "(R=0.000000,G=0.660000,B=1.000000,A=1.000000)" 1e+01)
  (Class|ImageWriteBlueprintLibrary|ExporttoDisk _output_get_2 _returnvalue_4 (Utilities|Struct|MakeImageWriteOptions "PNG" (delegate Custom|OnComplete))))

(fn ConstructionScript)