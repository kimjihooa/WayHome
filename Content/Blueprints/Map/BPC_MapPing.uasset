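; Actor component that shows a minimap icon for its owning actor.
; When the HUD signals map widget creation, it creates a WB_MiniMapCheckpoint with the configured icon settings, adds it to the viewport and registers it in the HUD's checkpoint list.
; Tick feeds the widget the owner's 2D offset from the player character.
; Wrapper events change icon texture, size and visibility; owner destruction removes the list entry by stored index, leaving the widget itself untouched.
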(event Custom|ChangeIconTexture
  (params (Texture :type Texture%202D%20Object%20Reference))
  (bind _minimapcheckpointwidget (Variables|Default|GetMinimapCheckpointWidget))
  ;[1 1 1] Custom Settings Wrapper
  (Utilities|IsValid _minimapcheckpointwidget
    (:Is%20Valid
      (Default|ChangeIcon _minimapcheckpointwidget Texture))
    (:Is%20Not%20Valid
      (Development|PrintString "Checkpoint Widget Not Valid"))))

(event Custom|ChangeIconSize
  (params (InSize :type Vector%202D%20Structure))
  (bind _minimapcheckpointwidget (Variables|Default|GetMinimapCheckpointWidget))
  ;[1 1 1] Custom Settings Wrapper
  (Utilities|IsValid _minimapcheckpointwidget
    (:Is%20Valid
      (Default|ChangeSize _minimapcheckpointwidget InSize))
    (:Is%20Not%20Valid
      (Development|PrintString "Checkpoint Widget Not Valid"))))

(event Custom|OnDestroyed
  (params (DestroyedActor :type Actor%20Object%20Reference))
  (Utilities|Array|RemoveIndex (Variables|/Game/Blueprints/BP_HUD.BP_HUD_C|GetCheckpointWidgets (Variables|Default|GetHUD)) (Variables|Default|GetListIndex)))

(event Custom|CreateWidget
  (Utilities|IsValid (Variables|/Game/Blueprints/BP_HUD.BP_HUD_C|GetMinimapWidget (Variables|Default|GetHUD))
    (:Is%20Valid
      (Variables|Default|SetMinimapWidget (Variables|/Game/Blueprints/BP_HUD.BP_HUD_C|GetMinimapWidget (Variables|Default|GetHUD)))
      (bind _returnvalue (UserInterface|CreateWidget "/Game/Blueprints/Map/WB_MiniMapCheckpoint.WB_MiniMapCheckpoint_C" 0 (Variables|/Game/Blueprints/BP_HUD.BP_HUD_C|GetMinimapWidget (Variables|Default|GetHUD)) (Variables|Default|GetbShowIconOutside) (Variables|Default|GetIconTexture) (Variables|Default|GetIconSize)))
      (bind _output_get (Variables|Default|SetMinimapCheckpointWidget _returnvalue))
      (UserInterface|Viewport|AddtoViewport _output_get 0)
      (bind _returnvalue_2 (Utilities|Array|AddUnique (Variables|/Game/Blueprints/BP_HUD.BP_HUD_C|GetCheckpointWidgets (Variables|Default|GetHUD)) _output_get))
      (Variables|Default|SetListIndex _returnvalue_2))
    (:Is%20Not%20Valid
      (Development|PrintString "Minimap widget not created"))))

(event Custom|GetHUD
  (bind _asbp_hud (Utilities|Casting|CastToBP_HUD (HUD|GetHUD (Game|GetPlayerController 0))))
  (Variables|Default|SetHUD _asbp_hud)
  (EventDispatchers|BindEventtoOnMapWidgetCreated _asbp_hud (delegate Custom|CreateWidget)))

(event Custom|CustomEvent
  (bind _minimapcheckpointwidget (Variables|Default|GetMinimapCheckpointWidget))
  ;[1 1 1] Custom Settings Wrapper
  (Utilities|IsValid _minimapcheckpointwidget
    (:Is%20Valid
      (Widget|SetVisibility _minimapcheckpointwidget "Visible"))
    (:Is%20Not%20Valid
      (Development|PrintString "Checkpoint Widget Not Valid"))))

(event Custom|CustomEvent_1
  (bind _minimapcheckpointwidget (Variables|Default|GetMinimapCheckpointWidget))
  ;[1 1 1] Custom Settings Wrapper
  (Utilities|IsValid _minimapcheckpointwidget
    (:Is%20Valid
      (Widget|SetVisibility _minimapcheckpointwidget "Hidden"))
    (:Is%20Not%20Valid
      (Development|PrintString "Checkpoint Widget Not Valid"))))

(event EventBeginPlay
  (Game|BindEventtoOnDestroyed (Components|GetOwner) (delegate Custom|OnDestroyed))
  (CallFunction|GetHUD))

(event EventTick
  (params (DeltaSeconds :type Float%20%28single-precision%29))
  (bind _minimapcheckpointwidget (Variables|Default|GetMinimapCheckpointWidget))
  (Utilities|IsValid _minimapcheckpointwidget
    (:Is%20Valid
      (Default|UpdateIconLocation _minimapcheckpointwidget (Math|Conversions|ToVector2D(Vector) (- (Transformation|GetActorLocation (Components|GetOwner)) (Transformation|GetActorLocation (Game|GetPlayerCharacter 0))))))))