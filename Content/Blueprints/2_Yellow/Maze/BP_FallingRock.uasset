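; BP_FallingRock is a maze rock that plays a fall sequence on spawn, then travels along MoveDir.
; When the sequence finishes, a looping timer steps the actor forward without sweep until it nears the referenced Cliff along that axis.
; A character faster than ImpactLimit hitting the cube against its direction, within an angle threshold, halts the movement and unbinds the hit event.
; Nodes for stopping the sequence and enabling physics are left unconnected.
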(event Custom|OnForward
  (bind _returnvalue (Utilities|Time|SetTimerbyEvent (delegate Custom|GoForward) 0.01 true))
  (Variables|Default|SetMoveTimer _returnvalue))

(event Custom|OnSpawn
  (bind _returnvalue (Sequencer|Player|CreateLevelSequencePlayer "/Game/Blueprints/2_Yellow/Maze/LS_RockFall.LS_RockFall" (Utilities|Struct|MakeMovieSceneSequencePlaybackSettings false "(Value=0)" 1.0 0.0 false true false false false false false true)))
  (bind _output_get (Variables|Default|SetSequancePlayer _returnvalue))
  (Sequencer|Player|Play _output_get :!class /Script/MovieScene.MovieSceneSequencePlayer)
  (EventDispatchers|BindEventtoOnFinished _output_get (delegate Custom|OnForward))
  (Collision|BindEventtoOnComponentHit (Variables|Default|GetCube) (delegate Custom|OnHit)))

(event Custom|GoForward
  (bind _returnvalue (Transformation|GetActorLocation))
  (bind _movedir (Variables|Default|GetMoveDir))
  (bind _speed (Variables|Default|GetSpeed))
  (bind _returnvalue_2 (* _speed _movedir))
  (bind _returnvalue_3 (+ _returnvalue _returnvalue_2))
  (Transformation|SetActorLocation _returnvalue_3 false false)
  (if (< (Math|Vector|VectorLength (* (- _returnvalue_3 (Transformation|GetActorLocation (Variables|Default|GetCliff))) (Variables|Default|GetMoveDir))) 5.0)
    (Utilities|Time|ClearandInvalidateTimerbyHandle (Variables|Default|GetMoveTimer))))

(event Custom|OnHit
  (params (HitComponent :type Primitive%20Component%20Object%20Reference) (OtherActor :type Actor%20Object%20Reference) (OtherComp :type Primitive%20Component%20Object%20Reference) (NormalImpulse :type Vector) (Hit :type Hit%20Result%20Structure%20%28by%20ref%29))
  (bind _ascharacter (Utilities|Casting|CastToCharacter OtherActor))
  (if (and (> (Math|Vector|VectorLength (Variables|/Script/Engine.MovementComponent|GetVelocity (Variables|/Script/Engine.Character|GetCharacterMovement _ascharacter))) (Variables|Default|GetImpactLimit)) (< (Math|Trig|RadiansToDegrees (Math|Trig|Acos(Degrees) (Math|Vector|DotProduct (.Normal (Collision|BreakHitResult Hit)) (* (Variables|Default|GetMoveDir) -1.0)))) (Variables|Default|GetDirThreshold)))
    (Development|PrintString "Hello")
    (Collision|UnbindEventfromOnComponentHit (Variables|Default|GetCube) (delegate Custom|OnHit))
    (Utilities|Time|ClearandInvalidateTimerbyHandle (Variables|Default|GetMoveTimer))))

(event EventBeginPlay
  (CallFunction|OnSpawn)
  (Utilities|IsValid (Variables|Default|GetCliff)
    (:Is%20Not%20Valid
      (Development|PrintString "Cliff Not Set"))))

(fn ConstructionScript)