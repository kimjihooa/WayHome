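; A maze rock that rolls along a world X or Y axis when a character hits it faster than an impact limit.
; The hit normal snaps to an axis, then a line trace sets the stopping point and subtracts any hit BP_MazeWall's damage from rock health upfront.
; A looping timer moves it there, where it is destroyed at zero health or backs into the block middle via timeline and re-arms hit detection.
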(event Custom|OnRockHit
  (params (HitComponent :type Primitive%20Component%20Object%20Reference) (OtherActor :type Actor%20Object%20Reference) (OtherComp :type Primitive%20Component%20Object%20Reference) (NormalImpulse :type Vector) (Hit :type Hit%20Result%20Structure%20%28by%20ref%29))
  ;[1 1 1] Check Power and Angle
  (bind _ascharacter (Utilities|Casting|CastToCharacter OtherActor))
  (if (> (Math|Vector|VectorLength (Variables|/Script/Engine.MovementComponent|GetVelocity (Variables|/Script/Engine.Character|GetCharacterMovement _ascharacter))) (Variables|Default|GetImpactLimit))
    (Variables|Default|SetCharacterSpeed (Math|Vector|VectorLength (Variables|/Script/Engine.MovementComponent|GetVelocity (Variables|/Script/Engine.Character|GetCharacterMovement _ascharacter))))
    (bind (_bisinrange _movedir) (CallFunction|CheckDir (.Normal (Collision|BreakHitResult Hit))))
    (if _bisinrange
      (Collision|UnbindEventfromOnComponentHit (Variables|Default|GetCube) (delegate Custom|OnRockHit))
      (Variables|Default|SetMove%20Dir _movedir)
      (CallFunction|StartRoll))))

(event Custom|Roll
  (bind _returnvalue (Transformation|GetActorLocation))
  (bind _move_dir (Variables|Default|GetMove%20Dir))
  (bind _speed (Variables|Default|GetSpeed))
  (bind _returnvalue_2 (* _move_dir _speed))
  (bind _returnvalue_3 (+ _returnvalue _returnvalue_2))
  ;[1 1 1] Forward
  (Transformation|SetActorLocation _returnvalue_3 false false)
  (if (< (Math|Vector|Distance(Vector) _returnvalue_3 (Variables|Default|GetDestination)) (Variables|Default|GetDistanceThreshold))
    (Transformation|SetActorLocation (Variables|Default|GetDestination) false false)
    (Utilities|Time|ClearandInvalidateTimerbyHandle (Variables|Default|GetRollTimer))
    ;[1 0.177 0.187] Is Dead?
    (if (<= (Variables|Default|GetHealth) 0)
      (Actor|DestroyActor)
      (else
        ;[1 1 1] Backward
        (bind _newtrack_0 (Timeline|Back Play)
          (:Update
            (Transformation|SetActorLocation (+ (Variables|Default|GetDestination) (* _newtrack_0 (- (Variables|Default|GetDestinationToMiddle) (Variables|Default|GetDestination)))) false false))
          (:Finished
            ;[1 1 1] End
            (Variables|Default|SetbIsRolling false)
            (Collision|AssignOnComponentHit (Variables|Default|GetCube) (delegate Custom|OnRockHit))))))))

(event Custom|StartRoll
  (if (not (Variables|Default|GetbIsRolling))
    (Variables|Default|SetbIsRolling true)
    (bind _outhit (Collision|LineTraceByChannel (Transformation|GetActorLocation) (+ (Transformation|GetActorLocation) (* (Variables|Default|GetMove%20Dir) 1e+04)) "TraceTypeQuery1" false 0 "ForDuration"))
    (bind _asbp_maze_wall (Utilities|Casting|CastToBP_MazeWall (.HitActor (Collision|BreakHitResult _outhit)))
      (:then
        (CallFunction|UpdateHealth (Variables|/Game/Blueprints/2_Yellow/Maze/BP_MazeWall.BP_MazeWall_C|GetDeal _asbp_maze_wall)))
      (:CastFailed
        _))
    (Variables|Default|SetDestination (- (.Location (Collision|BreakHitResult _outhit)) (* (Variables|Default|GetMove%20Dir) (Variables|Default|GetRockHalfSize))))
    (Variables|Default|SetDestinationToMiddle (- (.Location (Collision|BreakHitResult _outhit)) (* (Variables|Default|GetMove%20Dir) (Variables|Default|GetBlockHalfSize))))
    (bind _returnvalue (Utilities|Time|SetTimerbyEvent (delegate Custom|Roll) 0.01 true))
    (Variables|Default|SetRollTimer _returnvalue)))

(event EventBeginPlay
  (Collision|BindEventtoOnComponentHit (Variables|Default|GetCube) (delegate Custom|OnRockHit)))

(fn ConstructionScript)

(fn CheckDir
  (params (ImpactDir :type Vector))
  (bind _returnvalue (Math|Vector|MakeVector 0.0 1.0 0.0))
  (bind _returnvalue_2 (Math|Vector|MakeVector 0.0 -1.0 0.0))
  (bind _returnvalue_3 (Math|Vector|MakeVector -1.0 0.0 0.0))
  (bind _returnvalue_4 (Math|Vector|MakeVector 1.0 0.0 0.0))
  (if (< (Math|Trig|RadiansToDegrees (Math|Trig|Acos(Degrees) (Math|Vector|DotProduct ImpactDir _returnvalue_3))) (Variables|Default|GetDirThreshold))
    (return true _returnvalue_3)
    (elif (< (Math|Trig|RadiansToDegrees (Math|Trig|Acos(Degrees) (Math|Vector|DotProduct ImpactDir _returnvalue_2))) (Variables|Default|GetDirThreshold))
      (return true _returnvalue_2)
      (elif (< (Math|Trig|RadiansToDegrees (Math|Trig|Acos(Degrees) (Math|Vector|DotProduct ImpactDir _returnvalue_4))) (Variables|Default|GetDirThreshold))
        (return true _returnvalue_4)
        (elif (< (Math|Trig|RadiansToDegrees (Math|Trig|Acos(Degrees) (Math|Vector|DotProduct ImpactDir _returnvalue))) (Variables|Default|GetDirThreshold))
          (return true _returnvalue)
          (else
            (return false "0, 0, 0")))))))

(fn UpdateHealth
  (params (Deal :type Integer))
  (Variables|Default|SetHealth (- (Variables|Default|GetHealth) Deal)))