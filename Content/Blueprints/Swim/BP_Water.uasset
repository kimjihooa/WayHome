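; Swimmable cartoon lake actor that styles its surface and underwater meshes by OceanType, with wave and look settings pushed to MPC_Lake and a dynamic material.
; While BP_Character overlaps the box, a looping timer measures depth and selects stand, surface or deep mode, adjusting movement and abilities.
; Repeater timers scale wading speed and jump, nudge surface height and trace for exit.
; Summed WaterAdder amounts raise the level by growing actor Z scale.
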(event OnComponentBeginOverlap(Box)
  (params (OverlappedComponent :type Primitive%20Component%20Object%20Reference) (OtherActor :type Actor%20Object%20Reference) (OtherComp :type Primitive%20Component%20Object%20Reference) (OtherBodyIndex :type Integer) (bFromSweep :type Boolean) (SweepResult :type Hit%20Result%20Structure%20%28by%20ref%29))
  (Utilities|FlowControl|Sequence
    (:then_0
      ;[0.3654 0.7546 1] Swimming
      (bind _asbp_character (Utilities|Casting|CastToBP_Character OtherActor))
      (Variables|Swim|SetCharacter _asbp_character)
      (Utilities|Time|UnpauseTimerbyHandle (Variables|Swim|GetDepthTrackerTimer))
      (Variables|/Script/WayHome.WHCharacter|SetbCanJump (Variables|Swim|GetCharacter) false)
      (Utilities|FlowControl|DoOnce false
        (:Completed
          (Variables|OriginalVars|SetOriginalSpeed (Variables|/Script/WayHome.WHCharacter|GetWalkSpeed (Variables|Swim|GetCharacter)))
          (Variables|OriginalVars|SetOriginalJumpZ (Variables|/Script/Engine.CharacterMovementComponent|GetJumpZVelocity (Variables|/Script/Engine.Character|GetCharacterMovement (Variables|Swim|GetCharacter))))
          (Variables|Swim.Stand|SetStandSpeed (Variables|/Script/Engine.CharacterMovementComponent|GetMaxSwimSpeed (Variables|/Script/Engine.Character|GetCharacterMovement (Variables|Swim|GetCharacter)))))))))

(event OnComponentEndOverlap(Box)
  (params (OverlappedComponent :type Primitive%20Component%20Object%20Reference) (OtherActor :type Actor%20Object%20Reference) (OtherComp :type Primitive%20Component%20Object%20Reference) (OtherBodyIndex :type Integer))
  (Utilities|FlowControl|Sequence
    (:then_0
      ;[0.3654 0.7546 1] Swimming
      (Utilities|Casting|CastToBP_Character OtherActor)
      (Utilities|Time|PauseTimerbyHandle (Variables|Swim|GetDepthTrackerTimer))
      (bind _returnvalue (Utilities|Time|SetTimerbyFunctionName 0 "SetOutModeRepeater" 0.1 true))
      (Variables|Swim.Out|SetOutTimer _returnvalue))))

(event Custom|RaiseLevel
  (bind _returnvalue (Transformation|GetActorScale3D))
  ;[0.4969 1 0.4002] RaiseLevel
  (if (> (Variables|Raise|GetRaiseNum) 0)
    (Transformation|SetActorScale3D (Math|Vector|MakeVector (.x _returnvalue) (.y _returnvalue) (+ (.z _returnvalue) (* (Variables|Raise|GetRaiseSpeed) (Variables|Raise|GetRaiseNum)))))))

(event Custom|SwimModeChanged
  ;[0.5021 0.869 1] Swimming
)

(event EventBeginPlay
  ;[0.3281 0.3281 0.3281] Material
  (CallFunction|WaterParameters)
  ;[0.5021 0.869 1] Swimming
  (bind _returnvalue (Utilities|Time|SetTimerbyFunctionName 0 "TrackDepth" 0.1 true))
  (bind _output_get (Variables|Swim|SetDepthTrackerTimer _returnvalue))
  (Utilities|Time|PauseTimerbyHandle _output_get)
  (EventDispatchers|BindEventtoOnSwimModeChanged (delegate Custom|SwimModeChanged))
  ;[0.4969 1 0.4002] RaiseLevel
  (bind _returnvalue_2 (Utilities|Time|SetTimerbyEvent (delegate Custom|RaiseLevel) 0.01 true))
  (Variables|Raise|SetLevelTimer _returnvalue_2)
  (for _array_element (Variables|Raise|GetWaterAdder)
    (Variables|Raise|SetRaiseNum (+ (Variables|/Game/Blueprints/3_Navy/BP_WaterAdder.BP_WaterAdder_C|GetAddAmount _array_element) (Variables|Raise|GetRaiseNum)))))

(event EventTick
  (params (DeltaSeconds :type Float%20%28single-precision%29))
  ;[0.3281 0.3281 0.3281] Material
  (if (Variables|GlobalParameters|GetUpdate%20WaterMesh%20Transform%20Runtime)
    (Rendering|Material|SetScalarParameterValue "/Game/Money/CartoonWaterShader/Materials/MaterialCollections/MPC_Lake.MPC_Lake" "Ocean Level" (.z (Transformation|GetWorldLocation (Variables|Default|GetCartoonWater))) :!class /Script/Engine.KismetMaterialLibrary)))

(fn ConstructionScript
  (bind _ocean_type (Variables|GlobalParameters|GetOcean%20Type))
  (bind _custom_lake_depth_material (Variables|CustomMaterials|GetCustom%20Lake%20Depth%20Material))
  (bind _cartoonwaterdepth (Variables|Default|GetCartoonWaterDepth))
  (Utilities|FlowControl|Sequence
    (:then_0
      (bind _returnvalue (Rendering|Material|CreateDynamicMaterialInstance (Variables|Default|GetCartoonWater) 0 (Utilities|Select :Index _ocean_type :NewEnumerator55 "/Game/Money/CartoonWaterShader/Materials/Water/Lake/MI_Lake_UNLIT_Transparent_NonTessellated.MI_Lake_UNLIT_Transparent_NonTessellated" :NewEnumerator56 "/Game/Money/CartoonWaterShader/Materials/Water/Lake/MI_Lake_UNLIT_NonTransparent_NonTessellated.MI_Lake_UNLIT_NonTransparent_NonTessellated" :NewEnumerator57 0 :NewEnumerator60 "/Game/Money/CartoonWaterShader/Materials/Water/Lake/MI_Lake_PBR_Transparent_NonTessellated.MI_Lake_PBR_Transparent_NonTessellated" :NewEnumerator61 "/Game/Money/CartoonWaterShader/Materials/Water/Lake/MI_Lake_PBR_NonTransparent_NonTessellated.MI_Lake_PBR_NonTransparent_NonTessellated" :NewEnumerator62 0 :NewEnumerator63 "/Game/Money/CartoonWaterShader/Materials/Water/Lake/MI_Lake_Mobile_Transparent.MI_Lake_Mobile_Transparent" :NewEnumerator64 "/Game/Money/CartoonWaterShader/Materials/Water/Lake/MI_Lake_Mobile_NonTransparent.MI_Lake_Mobile_NonTransparent" :NewEnumerator65 0 :NewEnumerator66 0) "None" :!class /Script/Engine.PrimitiveComponent))
      (bind _output_get (Variables|Default|SetCurrent%20Material%20 _returnvalue))
      (Rendering|Material|SetMaterial (Variables|Default|GetCartoonWater) 0 _output_get)
      (switch Utilities|FlowControl|Switch|SwitchonOceanType _ocean_type
        (:NewEnumerator55
          (bind _returnvalue_2 (Rendering|Material|CreateDynamicMaterialInstance _cartoonwaterdepth 0 "/Game/Money/CartoonWaterShader/Materials/Water/Lake/MI_Lake_NoTessellation_Depth.MI_Lake_NoTessellation_Depth" "None" :!class /Script/Engine.PrimitiveComponent :!label _label))
          (bind _output_get_2 (Variables|Default|SetCurrent%20Depth%20Material%20 _returnvalue_2))
          (Rendering|Material|SetMaterial (Variables|Default|GetCartoonWaterDepth) 0 _output_get_2)
          (Rendering|Material|SetMaterial (Variables|Default|GetUnderwater) 0 _output_get_2)
          (Rendering|Material|SetMaterial (Variables|Default|GetUnderwaterSide) 0 _output_get_2)
          (Rendering|Material|SetMaterial (Variables|Default|GetUnderwaterSide2) 0 _output_get_2)
          (Rendering|Material|SetMaterial (Variables|Default|GetUnderwaterSide3) 0 _output_get_2)
          (Rendering|Material|SetMaterial (Variables|Default|GetUnderwaterSide4) 0 _output_get_2))
        (:NewEnumerator56
          (goto _label))
        (:NewEnumerator60
          (goto _label))
        (:NewEnumerator61
          (goto _label))
        (:NewEnumerator63
          (Rendering|SetVisibility _cartoonwaterdepth false false :!label _label_2)
          (Rendering|SetVisibility (Variables|Default|GetUnderwater) false false)
          (Rendering|SetVisibility (Variables|Default|GetUnderwaterSide) false false)
          (Rendering|SetVisibility (Variables|Default|GetUnderwaterSide2) false false)
          (Rendering|SetVisibility (Variables|Default|GetUnderwaterSide3) false false)
          (Rendering|SetVisibility (Variables|Default|GetUnderwaterSide4) false false))
        (:NewEnumerator64
          (goto _label_2))
        (:NewEnumerator66
          (Rendering|Material|SetMaterial (Variables|Default|GetCartoonWater) 0 (Variables|CustomMaterials|GetCustom%20Lake%20Material))
          (Rendering|Material|SetMaterial (Variables|Default|GetCartoonWaterDepth) 0 _custom_lake_depth_material)
          (Rendering|Material|SetMaterial (Variables|Default|GetUnderwater) 0 _custom_lake_depth_material)
          (Rendering|Material|SetMaterial (Variables|Default|GetUnderwaterSide) 0 _custom_lake_depth_material)
          (Rendering|Material|SetMaterial (Variables|Default|GetUnderwaterSide2) 0 _custom_lake_depth_material)
          (Rendering|Material|SetMaterial (Variables|Default|GetUnderwaterSide3) 0 _custom_lake_depth_material)
          (Rendering|Material|SetMaterial (Variables|Default|GetUnderwaterSide4) 0 _custom_lake_depth_material))))
    (:then_1
      (CallFunction|WaterParameters))))

(fn SetSwimMode
  (params (Depth :type Float%20%28double-precision%29))
  (bind _character (Variables|Swim|GetCharacter))
  (bind _charactermovement (Variables|/Script/Engine.Character|GetCharacterMovement _character))
  (if (< Depth (Variables|Swim.Stand|GetStandOffset))
    (if (!= (Variables|Swim|GetSwimMode) 1)
      (Variables|Swim|SetSwimMode "NewEnumerator1")
      (Swim|SetStandMode _charactermovement)
      (Default|CallOnSwimModeChanged :!label _label))
    (elif (> Depth (- (Components|Capsule|GetScaledCapsuleHalfHeight (Variables|/Script/Engine.Character|GetCapsuleComponent (Variables|Swim|GetCharacter))) (Variables|Swim.Deep|GetDeepOffset)))
      (if (!= (Variables|Swim|GetSwimMode) 3)
        (Variables|Swim|SetSwimMode "NewEnumerator3")
        (Swim|SetDeepMode _charactermovement)
        (goto _label))
      (elif (!= (Variables|Swim|GetSwimMode) 2)
        (Variables|Swim|SetSwimMode "NewEnumerator2")
        (Swim|SetSurfaceMode _charactermovement)
        (goto _label)))))

(fn SetOutMode
  (params (Movement :type Character%20Movement%20Component%20Object%20Reference))
  (bind _character (Variables|Swim|GetCharacter))
  (Variables|/Script/Engine.CharacterMovementComponent|SetMaxWalkSpeed Movement (Variables|OriginalVars|GetOriginalSpeed))
  (Variables|/Script/Engine.CharacterMovementComponent|SetJumpZVelocity Movement (Variables|OriginalVars|GetOriginalJumpZ))
  (Pawn|Components|CharacterMovement|SetMovementMode Movement "MOVE_Walking" 0)
  (Variables|/Script/Engine.PhysicsVolume|SetbWaterVolume (Class|MovementComponent|GetPhysicsVolume Movement) false)
  (Variables|/Script/Engine.CharacterMovementComponent|SetGravityScale Movement 1.0)
  (Variables|/Script/WayHome.WHCharacter|SetbCanJump _character true)
  (Variables|/Script/WayHome.WHCharacter|SetbCanAscend _character false)
  (Variables|/Script/WayHome.WHCharacter|SetbCanDescend _character false)
  (Variables|/Script/WayHome.WHCharacter|SetbCanSprint _character true)
  (Variables|/Script/WayHome.WHCharacter|SetbCanCrouch _character true))

(fn SetOutModeRepeater
  (bind _outhit (Collision|LineTraceByChannel (Transformation|GetActorLocation (Variables|Swim|GetCharacter)) (+ (Transformation|GetActorLocation (Variables|Swim|GetCharacter)) "0.000000,0.000000,-1000.000000") "TraceTypeQuery1" false (Utilities|Array|MakeArray (Variables|Swim|GetCharacter)) "None" false))
  (if (!= (.HitActor (Collision|BreakHitResult _outhit)) self)
    (Utilities|Time|ClearandInvalidateTimerbyHandle (Variables|Swim.Out|GetOutTimer))
    (Utilities|Time|ClearandInvalidateTimerbyHandle (Variables|Swim.Stand|GetStandTimer))
    (Utilities|Time|ClearandInvalidateTimerbyHandle (Variables|Swim.Surface|GetSurfaceTimer))
    (if (!= (Variables|Swim|GetSwimMode) 0)
      (Variables|Swim|SetSwimMode "NewEnumerator0")
      (Swim|SetOutMode (Variables|/Script/Engine.Character|GetCharacterMovement (Variables|Swim|GetCharacter)))
      (Variables|Swim|SetCharacter 0)
      (Default|CallOnSwimModeChanged))))

(fn SetStandMode
  (params (Movement :type Character%20Movement%20Component%20Object%20Reference))
  (bind _character (Variables|Swim|GetCharacter))
  (Utilities|Time|ClearandInvalidateTimerbyHandle (Variables|Swim.Out|GetOutTimer))
  (Utilities|Time|ClearandInvalidateTimerbyHandle (Variables|Swim.Stand|GetStandTimer))
  (Utilities|Time|ClearandInvalidateTimerbyHandle (Variables|Swim.Surface|GetSurfaceTimer))
  (Variables|/Script/WayHome.WHCharacter|SetbCanSprint _character false)
  (Variables|/Script/WayHome.WHCharacter|SetbCanCrouch _character false)
  (Variables|/Game/Blueprints/Character/BP_Character.BP_Character_C|SetbCanAscend _character false)
  (Variables|/Script/WayHome.WHCharacter|SetbCanDescend _character false)
  (Variables|/Script/Engine.CharacterMovementComponent|SetGravityScale Movement 1.0)
  (bind _returnvalue (Utilities|Time|SetTimerbyFunctionName 0 "SetStandModeRepeater" 0.1 true))
  (Variables|Swim.Stand|SetStandTimer _returnvalue)
  (Pawn|Components|CharacterMovement|SetMovementMode Movement "MOVE_Falling" 0)
  (Variables|/Script/Engine.PhysicsVolume|SetbWaterVolume (Class|MovementComponent|GetPhysicsVolume Movement) false))

(fn SetStandModeRepeater
  (bind _character (Variables|Swim|GetCharacter))
  (bind _depth (Variables|Swim|GetDepth))
  (bind _character_2 (Variables|Swim|GetCharacter))
  (bind _returnvalue (Math|Float|Absolute(Float) _depth))
  (bind _capsulecomponent (Variables|/Script/Engine.Character|GetCapsuleComponent _character_2))
  (bind _charactermovement (Variables|/Script/Engine.Character|GetCharacterMovement _character))
  (bind _returnvalue_2 (Components|Capsule|GetScaledCapsuleHalfHeight _capsulecomponent))
  (bind _returnvalue_3 (/ _returnvalue _returnvalue_2))
  (Variables|/Script/Engine.CharacterMovementComponent|SetMaxWalkSpeed _charactermovement (+ (Variables|Swim.Stand|GetStandSpeed) (* (- (Variables|OriginalVars|GetOriginalSpeed) (Variables|Swim.Stand|GetStandSpeed)) _returnvalue_3)))
  (if (> _returnvalue_3 (Variables|Swim.Stand|GetJumpBlock))
    (if (< (Math|Float|Absolute(Float) (.z (Variables|/Script/Engine.MovementComponent|GetVelocity _charactermovement))) 5.0)
      (Variables|/Script/Engine.CharacterMovementComponent|SetJumpZVelocity _charactermovement (* (Variables|OriginalVars|GetOriginalJumpZ) _returnvalue_3))
      (Variables|/Script/WayHome.WHCharacter|SetbCanJump (Variables|Swim|GetCharacter) true))
    (else
      (Variables|/Script/WayHome.WHCharacter|SetbCanJump (Variables|Swim|GetCharacter) false))))

(fn WaterParameters
  (bind _current_material_ (Variables|Default|GetCurrent%20Material%20))
  (bind _current_material__2 (Variables|Default|GetCurrent%20Material%20))
  (bind _current_material__3 (Variables|Default|GetCurrent%20Material%20))
  (bind _current_material__4 (Variables|Default|GetCurrent%20Material%20))
  (bind _current_material__5 (Variables|Default|GetCurrent%20Material%20))
  (bind _current_material__6 (Variables|Default|GetCurrent%20Material%20))
  (bind _current_material__7 (Variables|Default|GetCurrent%20Material%20))
  (bind _current_material__8 (Variables|Default|GetCurrent%20Material%20))
  (bind _current_material__9 (Variables|Default|GetCurrent%20Material%20))
  (bind _current_material__10 (Variables|Default|GetCurrent%20Material%20))
  (bind _current_material__11 (Variables|Default|GetCurrent%20Material%20))
  (Utilities|FlowControl|Sequence
    (:then_0
      ;[1 1 1] Global Parameters
      (Rendering|Material|SetScalarParameterValue "/Game/Money/CartoonWaterShader/Materials/MaterialCollections/MPC_Lake.MPC_Lake" "Wave Speed Global" (Variables|GlobalParameters|GetWave%20Speed) :!class /Script/Engine.KismetMaterialLibrary)
      (Rendering|Material|SetScalarParameterValue _current_material__7 "Global Opacity" (Variables|GlobalParameters|GetGlobal%20Opacity) :!class /Script/Engine.MaterialInstanceDynamic)
      (Rendering|Material|SetScalarParameterValue "/Game/Money/CartoonWaterShader/Materials/MaterialCollections/MPC_Lake.MPC_Lake" "Day Intensity" (Variables|GlobalParameters|GetDay%20Intensity) :!class /Script/Engine.KismetMaterialLibrary)
      (Rendering|Material|SetScalarParameterValue _current_material__7 "Water Depth" (Variables|GlobalParameters|GetWater%20Depth) :!class /Script/Engine.MaterialInstanceDynamic)
      (Rendering|Material|SetScalarParameterValue _current_material__7 "Sun Reflection Intensity" (Variables|GlobalParameters|GetSun%20Reflection%20Intensity) :!class /Script/Engine.MaterialInstanceDynamic)
      (Rendering|Material|SetScalarParameterValue _current_material__7 "Sun Reflection Tightness" (Variables|GlobalParameters|GetSun%20Reflection%20Tightness) :!class /Script/Engine.MaterialInstanceDynamic)
      (Rendering|Material|SetScalarParameterValue _current_material__7 "Shore Distance" (Variables|GlobalParameters|GetShore%20Distance) :!class /Script/Engine.MaterialInstanceDynamic)
      (Rendering|Material|SetScalarParameterValue "/Game/Money/CartoonWaterShader/Materials/MaterialCollections/MPC_Lake.MPC_Lake" "Tesselation Factor" (Variables|GlobalParameters|GetTessellation%20Factor) :!class /Script/Engine.KismetMaterialLibrary))
    (:then_1
      ;[1 1 1] Gerstner Waves
      (Rendering|Material|SetScalarParameterValue "/Game/Money/CartoonWaterShader/Materials/MaterialCollections/MPC_Lake.MPC_Lake" "Wave Length" (Variables|GerstnerWave|GetWave%20Length) :!class /Script/Engine.KismetMaterialLibrary)
      (Rendering|Material|SetScalarParameterValue "/Game/Money/CartoonWaterShader/Materials/MaterialCollections/MPC_Lake.MPC_Lake" "Amplitude" (Variables|GerstnerWave|GetAmplitude) :!class /Script/Engine.KismetMaterialLibrary)
      (Rendering|Material|SetScalarParameterValue "/Game/Money/CartoonWaterShader/Materials/MaterialCollections/MPC_Lake.MPC_Lake" "Steepness" (Variables|GerstnerWave|GetSteepness) :!class /Script/Engine.KismetMaterialLibrary)
      (Rendering|Material|SetScalarParameterValue "/Game/Money/CartoonWaterShader/Materials/MaterialCollections/MPC_Lake.MPC_Lake" "Gerstner Wave Speed " (Variables|GerstnerWave|GetGerstner%20Wave%20Speed%20) :!class /Script/Engine.KismetMaterialLibrary)
      (Rendering|Material|SetScalarParameterValue "/Game/Money/CartoonWaterShader/Materials/MaterialCollections/MPC_Lake.MPC_Lake" "Wind Direction" (Variables|GerstnerWave|GetWind%20Direction) :!class /Script/Engine.KismetMaterialLibrary))
    (:then_2
      ;[1 1 1] Distances
      (Rendering|Material|SetScalarParameterValue _current_material__11 "Color Distance Fade" (Variables|Distances|GetColor%20Distance%20Fade) :!class /Script/Engine.MaterialInstanceDynamic)
      (Rendering|Material|SetScalarParameterValue _current_material__11 "Color Distance Falloff" (Variables|Distances|GetColor%20Distance%20Falloff) :!class /Script/Engine.MaterialInstanceDynamic)
      (Rendering|Material|SetScalarParameterValue _current_material__11 "Water Depth Distance Fade" (Variables|Distances|GetWater%20Depth%20Distance%20Fade) :!class /Script/Engine.MaterialInstanceDynamic)
      (Rendering|Material|SetScalarParameterValue _current_material__11 "Water Depth Distance Falloff" (Variables|Distances|GetWater%20Depth%20Distance%20Falloff) :!class /Script/Engine.MaterialInstanceDynamic)
      (Rendering|Material|SetScalarParameterValue _current_material__11 "Foam Distance Fade" (Variables|Distances|GetFoam%20Distance%20Fade) :!class /Script/Engine.MaterialInstanceDynamic)
      (Rendering|Material|SetScalarParameterValue _current_material__11 "Foam Distance Falloff" (Variables|Distances|GetFoam%20Distance%20Falloff) :!class /Script/Engine.MaterialInstanceDynamic)
      (Rendering|Material|SetScalarParameterValue _current_material__11 "Normal Distance Fade" (Variables|Distances|GetNormal%20Distance%20Fade) :!class /Script/Engine.MaterialInstanceDynamic)
      (Rendering|Material|SetScalarParameterValue _current_material__11 "Normal Distance Falloff" (Variables|Distances|GetNormal%20Distance%20Falloff) :!class /Script/Engine.MaterialInstanceDynamic)
      (Rendering|Material|SetScalarParameterValue _current_material__11 "Refraction Distance Fade" (Variables|Distances|GetRefraction%20Distance%20Fade) :!class /Script/Engine.MaterialInstanceDynamic)
      (Rendering|Material|SetScalarParameterValue _current_material__11 "Refraction Distance Falloff" (Variables|Distances|GetRefraction%20Distance%20Falloff) :!class /Script/Engine.MaterialInstanceDynamic)
      (Rendering|Material|SetScalarParameterValue _current_material__11 "SSS Distance Fade" (Variables|Distances|GetSSS%20Distance%20Fade) :!class /Script/Engine.MaterialInstanceDynamic)
      (Rendering|Material|SetScalarParameterValue _current_material__11 "SSS Distance Falloff" (Variables|Distances|GetSSS%20Distance%20Falloff) :!class /Script/Engine.MaterialInstanceDynamic))
    (:then_3
      ;[1 1 1] Normals
      (Rendering|Material|SetScalarParameterValue _current_material__10 "Small Normal Speed" (Variables|Normals|GetSmall%20Normal%20Speed) :!class /Script/Engine.MaterialInstanceDynamic)
      (Rendering|Material|SetScalarParameterValue _current_material__10 "Small Normal Intensity" (Variables|Normals|GetSmall%20Normal%20Intensity) :!class /Script/Engine.MaterialInstanceDynamic)
      (Rendering|Material|SetScalarParameterValue _current_material__10 "Small Normal Tiling" (Variables|Normals|GetSmall%20Normal%20Tiling) :!class /Script/Engine.MaterialInstanceDynamic)
      (Rendering|Material|SetScalarParameterValue _current_material__10 "Large Normal Speed" (Variables|Normals|GetLarge%20Normal%20Speed) :!class /Script/Engine.MaterialInstanceDynamic)
      (Rendering|Material|SetScalarParameterValue _current_material__10 "Large Normal Intensity" (Variables|Normals|GetLarge%20Normal%20Intensity) :!class /Script/Engine.MaterialInstanceDynamic)
      (Rendering|Material|SetScalarParameterValue _current_material__10 "Large Normal Tiling" (Variables|Normals|GetLarge%20Normal%20Tiling) :!class /Script/Engine.MaterialInstanceDynamic))
    (:then_4
      ;[1 1 1] Seafoam
      (Rendering|Material|SetScalarParameterValue _current_material__9 "Seafoam Intensity" (Variables|Seafoam|GetSeafoam%20Intensity) :!class /Script/Engine.MaterialInstanceDynamic)
      (Rendering|Material|SetScalarParameterValue _current_material__9 "Seafoam Base Height" (Variables|Seafoam|GetSeafoam%20Base%20Height) :!class /Script/Engine.MaterialInstanceDynamic)
      (Rendering|Material|SetScalarParameterValue _current_material__9 "Seafoam Softness" (Variables|Seafoam|GetSeafoam%20Softness) :!class /Script/Engine.MaterialInstanceDynamic)
      (Rendering|Material|SetScalarParameterValue _current_material__9 "Seafoam Distorsion" (Variables|Seafoam|GetSeafoam%20Distorsion) :!class /Script/Engine.MaterialInstanceDynamic)
      (Rendering|Material|SetScalarParameterValue _current_material__9 "Seafoam Tiling" (Variables|Seafoam|GetSeafoam%20Tiling) :!class /Script/Engine.MaterialInstanceDynamic))
    (:then_5
      ;[1 1 1] Foam
      (Rendering|Material|SetScalarParameterValue _current_material__8 "Foam Intensity" (Variables|Foam|GetFoam%20Intensity) :!class /Script/Engine.MaterialInstanceDynamic)
      (Rendering|Material|SetScalarParameterValue _current_material__8 "Foam Speed" (Variables|Foam|GetFoam%20Speed) :!class /Script/Engine.MaterialInstanceDynamic)
      (Rendering|Material|SetScalarParameterValue _current_material__8 "Foam X Tile" (Variables|Foam|GetFoam%20X%20Tile) :!class /Script/Engine.MaterialInstanceDynamic)
      (Rendering|Material|SetScalarParameterValue _current_material__8 "Foam Y Tile" (Variables|Foam|GetFoam%20Y%20Tile) :!class /Script/Engine.MaterialInstanceDynamic)
      (Rendering|Material|SetScalarParameterValue _current_material__8 "Intersection Size" (Variables|Foam|GetIntersection%20Size) :!class /Script/Engine.MaterialInstanceDynamic)
      (Rendering|Material|SetScalarParameterValue _current_material__8 "Intersection Softness" (Variables|Foam|GetIntersection%20Softness) :!class /Script/Engine.MaterialInstanceDynamic)
      (Rendering|Material|SetScalarParameterValue _current_material__8 "Intersection Size Reduction Over Distance" (Variables|Foam|GetIntersection%20Size%20Reduction%20Over%20Distance) :!class /Script/Engine.MaterialInstanceDynamic))
    (:then_6
      ;[1 1 1] Cubemap
      (Rendering|Material|SetScalarParameterValue _current_material__6 "CubeMap Intensity" (Variables|Reflection|GetCubeMap%20Intensity) :!class /Script/Engine.MaterialInstanceDynamic)
      (Rendering|Material|SetScalarParameterValue _current_material__6 "Reflection Angle" (Variables|Reflection|GetReflection%20Angle) :!class /Script/Engine.MaterialInstanceDynamic)
      (Rendering|Material|SetScalarParameterValue _current_material__6 "Specular Intensity" (Variables|Reflection|GetSpecular%20Intensity) :!class /Script/Engine.MaterialInstanceDynamic))
    (:then_7
      ;[1 1 1] Refraction
      (Rendering|Material|SetScalarParameterValue (Variables|Default|GetCurrent%20Material%20) "Refraction Amount" (Variables|Refraction|GetRefraction%20Amount) :!class /Script/Engine.MaterialInstanceDynamic))
    (:then_8
      ;[1 1 1] Highlight
      (Rendering|Material|SetScalarParameterValue _current_material__4 "Highlight Intensity" (Variables|Highlight|GetHighlight%20Intensity) :!class /Script/Engine.MaterialInstanceDynamic)
      (Rendering|Material|SetScalarParameterValue _current_material__4 "Highlight Base Height" (Variables|Highlight|GetHighlight%20Base%20Height) :!class /Script/Engine.MaterialInstanceDynamic)
      (Rendering|Material|SetScalarParameterValue _current_material__4 "Highlight Softness" (Variables|Highlight|GetHighlight%20Softness) :!class /Script/Engine.MaterialInstanceDynamic)
      (Rendering|Material|SetScalarParameterValue _current_material__4 "Highlight Density" (Variables|Highlight|GetHighlight%20Density) :!class /Script/Engine.MaterialInstanceDynamic))
    (:then_9
      ;[1 1 1] Trough
      (Rendering|Material|SetScalarParameterValue _current_material__3 "Trough Intensity" (Variables|Trough|GetTrough%20Intensity) :!class /Script/Engine.MaterialInstanceDynamic)
      (Rendering|Material|SetScalarParameterValue _current_material__3 "Trough Base Height" (Variables|Trough|GetTrough%20Base%20Height) :!class /Script/Engine.MaterialInstanceDynamic)
      (Rendering|Material|SetScalarParameterValue _current_material__3 "Trough Softness" (Variables|Trough|GetTrough%20Softnes) :!class /Script/Engine.MaterialInstanceDynamic))
    (:then_10
      ;[1 1 1] SSS
      (Rendering|Material|SetScalarParameterValue _current_material__2 "SSS Intensity" (Variables|SubsurfaceScattering|GetSSS%20Intensity) :!class /Script/Engine.MaterialInstanceDynamic)
      (Rendering|Material|SetScalarParameterValue _current_material__2 "SSS Base Height" (Variables|SubsurfaceScattering|GetSSS%20Base%20Height) :!class /Script/Engine.MaterialInstanceDynamic)
      (Rendering|Material|SetScalarParameterValue _current_material__2 "SSS Softness" (Variables|SubsurfaceScattering|GetSSS%20Softness) :!class /Script/Engine.MaterialInstanceDynamic))
    (:then_11
      ;[1 1 1] Colors
      (Rendering|Material|SetVectorParameterValue _current_material_ "Base Color" (Variables|Colors|GetBase%20Color) :!class /Script/Engine.MaterialInstanceDynamic)
      (Rendering|Material|SetVectorParameterValue _current_material_ "Far Color" (Variables|Colors|GetFar%20Color) :!class /Script/Engine.MaterialInstanceDynamic)
      (Rendering|Material|SetVectorParameterValue _current_material_ "Shallow Water Color" (Variables|Colors|GetShallow%20Water%20Color) :!class /Script/Engine.MaterialInstanceDynamic)
      (Rendering|Material|SetVectorParameterValue _current_material_ "Trough Color" (Variables|Colors|GetTrough%20Color) :!class /Script/Engine.MaterialInstanceDynamic)
      (Rendering|Material|SetVectorParameterValue _current_material_ "SSS Color" (Variables|Colors|GetSSS%20Color) :!class /Script/Engine.MaterialInstanceDynamic)
      (Rendering|Material|SetVectorParameterValue _current_material_ "Foam Color" (Variables|Colors|GetFoam%20Color) :!class /Script/Engine.MaterialInstanceDynamic)
      (Rendering|Material|SetVectorParameterValue _current_material_ "Seafoam Color" (Variables|Colors|GetSeafoam%20Color) :!class /Script/Engine.MaterialInstanceDynamic))
    (:then_12
      ;[1 1 1] Location Z
      (Rendering|Material|SetScalarParameterValue "/Game/Money/CartoonWaterShader/Materials/MaterialCollections/MPC_Lake.MPC_Lake" "Ocean Level" (.z (Transformation|GetWorldLocation (Variables|Default|GetCartoonWater))) :!class /Script/Engine.KismetMaterialLibrary)
      (Transformation|SetRelativeScale3D (Variables|Default|GetUnderwater) (Math|Vector|MakeVector 1.0 1.0 (Variables|Underwater|GetUnderwater%20Mesh%20Z%20scale))))
    (:then_13
      ;[1 1 1] Underwater
      (Rendering|Material|SetScalarParameterValue _current_material__5 "Refraction Amount Depth" (Variables|Underwater|GetRefraction%20Amount%20Depth) :!class /Script/Engine.MaterialInstanceDynamic)
      (Rendering|Material|SetScalarParameterValue _current_material__5 "Refraction Depth" (Variables|Underwater|GetRefraction%20Depth) :!class /Script/Engine.MaterialInstanceDynamic)
      (Rendering|Material|SetScalarParameterValue _current_material__5 "Underwater Opacity" (Variables|Underwater|GetUnderwater%20Opacity) :!class /Script/Engine.MaterialInstanceDynamic))))

(fn SetSurfaceMode
  (params (Movement :type Character%20Movement%20Component%20Object%20Reference))
  (bind _character (Variables|Swim|GetCharacter))
  (Utilities|Time|ClearandInvalidateTimerbyHandle (Variables|Swim.Out|GetOutTimer))
  (Utilities|Time|ClearandInvalidateTimerbyHandle (Variables|Swim.Stand|GetStandTimer))
  (Utilities|Time|ClearandInvalidateTimerbyHandle (Variables|Swim.Surface|GetSurfaceTimer))
  (Variables|/Game/Blueprints/Character/BP_Character.BP_Character_C|SetbCanAscend _character false)
  (Variables|/Script/WayHome.WHCharacter|SetbCanDescend _character false)
  (if (> (Variables|Swim|GetDepth) 0.0)
    (Variables|Swim.Surface|SetbHasToAscend true)
    (else
      (Variables|Swim.Surface|SetbHasToAscend false)))
  (if (> (.z (Variables|/Script/Engine.MovementComponent|GetVelocity Movement)) 0.0)
    (Variables|/Script/Engine.MovementComponent|SetVelocity Movement (Math|Vector|MakeVector (.x (Variables|/Script/Engine.MovementComponent|GetVelocity Movement)) (.y (Variables|/Script/Engine.MovementComponent|GetVelocity Movement)) 0.0)))
  (bind _returnvalue (Utilities|Time|SetTimerbyFunctionName 0 "SetSurfaceModeRepeater" (Variables|Swim.Surface|GetCounterForceInterval) true))
  (Variables|Swim.Surface|SetSurfaceTimer _returnvalue)
  (Pawn|Components|CharacterMovement|SetMovementMode Movement "MOVE_Swimming" 0)
  (Variables|/Script/Engine.PhysicsVolume|SetbWaterVolume (Class|MovementComponent|GetPhysicsVolume Movement) true)
  (Variables|/Script/Engine.CharacterMovementComponent|SetGravityScale Movement 0.0))

(fn SetSurfaceModeRepeater
  (bind _character (Variables|Swim|GetCharacter))
  (if (< (Math|Float|Absolute(Float) (- (Variables|Swim|GetDepth) (Variables|Swim.Surface|GetSurfaceOffset))) 1e+01)
    (Variables|/Game/Blueprints/Character/BP_Character.BP_Character_C|SetbCanAscend _character false)
    (Variables|/Script/WayHome.WHCharacter|SetbCanDescend _character true)
    (Utilities|Time|ClearandInvalidateTimerbyHandle (Variables|Swim.Surface|GetSurfaceTimer))
    (elif (Variables|Swim.Surface|GetbHasToAscend)
      (Transformation|AddActorWorldOffset (Variables|Swim|GetCharacter) (Math|Vector|MakeVector 0.0 0.0 (Variables|Swim.Surface|GetCounterZSpeed)))
      (else
        (bind _israising (CallFunction|GetIsRaising))
        (if (not _israising)
          (Transformation|AddActorWorldOffset (Variables|Swim|GetCharacter) (Math|Vector|MakeVector 0.0 0.0 (* (Variables|Swim.Surface|GetCounterZSpeed) -1.0))))))))

(fn SetDeepMode
  (params (Movement :type Character%20Movement%20Component%20Object%20Reference))
  (bind _character (Variables|Swim|GetCharacter))
  (Utilities|Time|ClearandInvalidateTimerbyHandle (Variables|Swim.Out|GetOutTimer))
  (Utilities|Time|ClearandInvalidateTimerbyHandle (Variables|Swim.Stand|GetStandTimer))
  (Utilities|Time|ClearandInvalidateTimerbyHandle (Variables|Swim.Surface|GetSurfaceTimer))
  (Pawn|Components|CharacterMovement|SetMovementMode Movement "MOVE_Swimming" 0)
  (Variables|/Script/Engine.PhysicsVolume|SetbWaterVolume (Class|MovementComponent|GetPhysicsVolume Movement) true)
  (Variables|/Game/Blueprints/Character/BP_Character.BP_Character_C|SetbCanAscend _character true)
  (Variables|/Script/WayHome.WHCharacter|SetbCanDescend _character true))

(fn TrackDepth
  (bind _character (Variables|Swim|GetCharacter))
  (Utilities|IsValid _character
    (:Is%20Valid
      (bind _output_get (Variables|Swim|SetDepth (+ (* (.z (Components|Box|GetScaledBoxExtent (Variables|Default|GetBox))) 2.0) (- (.z (Transformation|GetActorLocation)) (.z (Transformation|GetActorLocation _character))))))
      (Swim|SetSwimMode _output_get))))

(fn GetIsRaising
  (bind _raisenum (Variables|Raise|GetRaiseNum))
  (bind _returnvalue (!= _raisenum 0))
  (if _returnvalue
    _
    (else
      _))
  (return _returnvalue))